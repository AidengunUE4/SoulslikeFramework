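; SaveGame object in the Soulslike Framework that keeps a registry of the game's save slots.
; AddSlot adds a slot name to the list if it is not already present and records it as the last saved slot.
; Getter functions return the full slot list and the most recently saved slot.
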(fn `AddSlot`
  (params (SlotName :type String))
  ;[0.05098 0.05098 0.05098] Adds new save slot
  (if (not (`KismetArrayLibrary.Array_Contains` (`self.Slots`) SlotName))
    (`KismetArrayLibrary.Array_AddUnique` (`self.Slots`) SlotName))
  (set `self.LastSavedSlot` SlotName))

(fn `GetAllSlots`
  (returns (Slots :type "Array of String"))
  ;[0.05098 0.05098 0.05098] Returns all save slots
  (return (`self.Slots`)))

(fn `GetLastSaveSlot`
  (returns (Output :type String))
  ;[0.05098 0.05098 0.05098] Returns last save slot
  (return (`self.LastSavedSlot`)))