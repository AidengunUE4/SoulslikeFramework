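; B_SequenceActor is a spawnable world actor that plays a configured level sequence as a skippable cinematic.
; On BeginPlay it creates a sequence player, binds its finished event and starts playback.
; Any key shows a skip notification on the player HUD and arms skipping, after which the game menu input stops playback.
; Finishing, whether natural or skipped, calls the OnSequenceFinished notification and destroys the actor after a short timer.
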(event `self.ReceiveBeginPlay`
  ;[0.05098 0.05098 0.05098] Play relevant sequence first thing after being spawned. When finished, send relevant message and destroy the actor.
  (bind (_outactor _returnvalue) (`LevelSequencePlayer.CreateLevelSequencePlayer` (`self.SequenceToPlay`) (`self.Settings`)))
  (bind _output_get (set `self.ActiveSequencePlayer` _returnvalue))
  (add `MovieSceneSequencePlayer.OnFinished` _output_get (delegate `Event Finished`))
  (`MovieSceneSequencePlayer.Play` (`self.ActiveSequencePlayer`)))

(event `Event Finished`
  ;[0.05098 0.05098 0.05098] Play relevant sequence first thing after being spawned. When finished, send relevant message and destroy the actor.
  (`self.OnSequenceFinished`)
  (`KismetSystemLibrary.K2_SetTimerDelegate` (delegate `Event Destroy`) 0.1))

(event `Event Destroy`
  ;[0.05098 0.05098 0.05098] Play relevant sequence first thing after being spawned. When finished, send relevant message and destroy the actor.
  (`self.K2_DestroyActor`))

(event `EnhancedInput|/Game/SoulslikeFramework/Input/Actions/IA_AnyKey`
  (params (ActionValue :type Boolean) (ElapsedSeconds :type "Float (double-precision)") (TriggeredSeconds :type "Float (double-precision)") (InputAction :type "InputAction Object Reference" :default "/Game/SoulslikeFramework/Input/Actions/IA_AnyKey.IA_AnyKey"))
  ;[0.05098 0.05098 0.05098] When any key is pressed, show skip cinematic notification widget and allow skipping
  (:`Started`
    (`self.ActiveSequencePlayer`
      (:`then`
        (bind _w_hud (message `/Game/SoulslikeFramework/Blueprints/Interfaces/BPI_Controller.GetPlayerHUD` (`GameplayStatics.GetPlayerController` 0)))
        (`/Game/SoulslikeFramework/Widgets/HUD/W_HUD.Event ShowSkipCinematicNotification` _w_hud)
        (set `self.CanBeSkipped?` true))
      (:`else`))))

(event `EnhancedInput|/Game/SoulslikeFramework/Input/Actions/IA_GameMenu`
  (params (ActionValue :type Boolean) (ElapsedSeconds :type "Float (double-precision)") (TriggeredSeconds :type "Float (double-precision)") (InputAction :type "InputAction Object Reference" :default "/Game/SoulslikeFramework/Input/Actions/IA_GameMenu.IA_GameMenu"))
  ;[0.05098 0.05098 0.05098] IA_GameMenu (esc/special btn) to skip cinematic
  (:`Started`
    (`self.ActiveSequencePlayer`
      (:`then`
        (if (`self.CanBeSkipped?`)
          (if (`MovieSceneSequencePlayer.IsPlaying` (`self.ActiveSequencePlayer`))
            (`MovieSceneSequencePlayer.Stop` (`self.ActiveSequencePlayer`))
            (set `self.ActiveSequencePlayer` null)
            (`self.Event Finished`))))
      (:`else`))))

(fn `UserConstructionScript`)