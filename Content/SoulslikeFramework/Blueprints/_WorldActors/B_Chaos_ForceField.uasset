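; Chaos force field actor for breaking destructible geometry, built to sit on B_Soulslike_Character as a child actor component.
; Enable and disable events, driven by notifies, toggle actor tick.
; While ticking, it applies an external cluster strain field with a huge-magnitude, no-falloff radial falloff, sized and centered on its Sphere component.
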(event `/Game/SoulslikeFramework/Blueprints/Interfaces/BPI_DestructibleHelper.EnableChaosDestroy`
  ;[0.05098 0.05098 0.05098] Custom example implementation for Chaos force field. This actor is attached as a child actor component to B_Soulslike_Character.
  ; Tick gets enabled/disabled through notifies.
  (`self.SetActorTickEnabled` true))

(event `self.ReceiveTick`
  (params (DeltaSeconds :type "Float (single-precision)"))
  (bind _sphere (`self.Sphere`))
  ;[0.05098 0.05098 0.05098] Custom example implementation for Chaos force field. This actor is attached as a child actor component to B_Soulslike_Character.
  ; Tick gets enabled/disabled through notifies.
  (`FieldSystemComponent.ApplyPhysicsField` (`self.FieldSystemComponent`) true "Field_ExternalClusterStrain" null (`RadialFalloff.SetRadialFalloff` (`self.RadialFalloff`) 99999999.0 0.0 1.0 0.0 (`SphereComponent.GetScaledSphereRadius` _sphere) (`SceneComponent.K2_GetComponentLocation` _sphere) "Field_FallOff_None")))

(event `/Game/SoulslikeFramework/Blueprints/Interfaces/BPI_DestructibleHelper.DisableChaosDestroy`
  ;[0.05098 0.05098 0.05098] Custom example implementation for Chaos force field. This actor is attached as a child actor component to B_Soulslike_Character.
  ; Tick gets enabled/disabled through notifies.
  (`self.SetActorTickEnabled` false))

(fn `UserConstructionScript`)