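; Actor component in the Soulslike Framework that grants, tracks and removes buffs on its owner.
; Adding async-loads the class from a buff data asset, constructs a buff object, fires its granted event (preceded by removed when loading) and stores it in ActiveBuffs.
; Removal matches by data asset or tag, first or all, with a delayed variant for async-load races.
; Additions and removals are broadcast through OnBuffDetected.
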(event `Event TryAddBuff`
  (params (Buff :type "/Game/SoulslikeFramework/Data/Buffs/PDA_Buff Object Reference") (Rank :type Integer :default 1) (`IsLoading?` :type Boolean))
  ;[0.05098 0.05098 0.05098] Constructs Buff object from soft class reference, grants it to player, and tracks it
  (bind _class (`|LoadAssetClass` (`/Game/SoulslikeFramework/Data/Buffs/PDA_Buff.Class` Buff))
    (:`Completed`
      (bind _asbuff_object (castclass `/Game/SoulslikeFramework/Data/Buffs/Logic/B_Buff` _class))
      (bind _returnvalue (`|GenericCreateObject` _asbuff_object Rank Buff (`self.GetOwner`)))
      (if `IsLoading?`
        (`/Game/SoulslikeFramework/Data/Buffs/Logic/B_Buff.Event OnRemoved` _returnvalue))
      (`/Game/SoulslikeFramework/Data/Buffs/Logic/B_Buff.Event OnGranted` _returnvalue)
      (`KismetArrayLibrary.Array_Add` (`self.ActiveBuffs`) _returnvalue)
      (`self.OnBuffDetected` Buff true))))

(event `Event DelayedRemoveBuff`
  (params (DelayDuration :type "Float (single-precision)") (Buff :type "/Game/SoulslikeFramework/Data/Buffs/PDA_Buff Object Reference"))
  ;[0.05098 0.05098 0.05098] Delayed version for removing target buff. Useful for combatting race conditions related to async loading.
  (`KismetSystemLibrary.Delay` DelayDuration)
  (for _array_element (`self.ActiveBuffs`)
    (bind _buffdata (`/Game/SoulslikeFramework/Data/Buffs/Logic/B_Buff.BuffData` _array_element)
      (:`then`
        (if (== _buffdata Buff)
          (set `self.Cache_Buff` _array_element)
          (break)))
      (:`else`)))
  (bind _cache_buff (`self.Cache_Buff`)
    (:`then`
      (`/Game/SoulslikeFramework/Data/Buffs/Logic/B_Buff.Event OnRemoved` _cache_buff)
      (`KismetArrayLibrary.Array_RemoveItem` (`self.ActiveBuffs`) _cache_buff)
      (`self.OnBuffDetected` null)
      (set `self.Cache_Buff` null))
    (:`else`)))

(fn `GetBuffsWithTag`
  (params (Tag :type "GameplayTag Structure"))
  (returns (Buffs :type "Array of /Game/SoulslikeFramework/Data/Buffs/Logic/B_Buff Object Reference"))
  (locals (LOCAL_Buffs :type "Array of /Game/SoulslikeFramework/Data/Buffs/Logic/B_Buff Object Reference"))
  ;[0.05098 0.05098 0.05098] Returns all buffs with tag
  (for _array_element (`self.ActiveBuffs`)
    (bind _buffdata (`/Game/SoulslikeFramework/Data/Buffs/Logic/B_Buff.BuffData` _array_element)
      (:`then`
        (if (== (`/Game/SoulslikeFramework/Data/Buffs/PDA_Buff.BuffTag` _buffdata) (`local.Tag`))
          (`KismetArrayLibrary.Array_Add` (`local.LOCAL_Buffs`) _array_element)))
      (:`else`)))
  (return (`local.LOCAL_Buffs`)))

(fn `RemoveAllBuffsOfType`
  (params (Buff :type "/Game/SoulslikeFramework/Data/Buffs/PDA_Buff Object Reference"))
  (locals (LOCAL_FoundBuff :type "/Game/SoulslikeFramework/Data/Buffs/Logic/B_Buff Object Reference"))
  ;[0.05098 0.05098 0.05098] Finds all buffs using the Buff data asset. Removes them from tracking array.
  (for _array_element (`self.ActiveBuffs`)
    (bind _buffdata (`/Game/SoulslikeFramework/Data/Buffs/Logic/B_Buff.BuffData` _array_element)
      (:`then`
        (if (== _buffdata Buff)
          (`/Game/SoulslikeFramework/Data/Buffs/Logic/B_Buff.Event OnRemoved` _array_element)
          (`KismetArrayLibrary.Array_RemoveItem` (`self.ActiveBuffs`) _array_element)
          (`self.OnBuffDetected` (`local.Buff`))))
      (:`else`))))

(fn `RemoveAllBuffsWithTag`
  (params (Tag :type "GameplayTag Structure"))
  ;[0.05098 0.05098 0.05098] Finds all the buffs using the Buff tag. Removes them and stops tracking.
  (bind _buffs (`self.GetBuffsWithTag` Tag))
  (for _array_element _buffs
    (`/Game/SoulslikeFramework/Data/Buffs/Logic/B_Buff.Event OnRemoved` _array_element)
    (`KismetArrayLibrary.Array_RemoveItem` (`self.ActiveBuffs`) _array_element)
    (`self.OnBuffDetected` (`/Game/SoulslikeFramework/Data/Buffs/Logic/B_Buff.BuffData` _array_element))))

(fn `RemoveBuffOfType`
  (params (Buff :type "/Game/SoulslikeFramework/Data/Buffs/PDA_Buff Object Reference"))
  (locals (LOCAL_FoundBuff :type "/Game/SoulslikeFramework/Data/Buffs/Logic/B_Buff Object Reference"))
  ;[0.05098 0.05098 0.05098] Finds the first buff using the Buff data asset. Removes it and stops tracking it.
  (for _array_element (`self.ActiveBuffs`)
    (bind _buffdata (`/Game/SoulslikeFramework/Data/Buffs/Logic/B_Buff.BuffData` _array_element)
      (:`then`
        (if (== _buffdata Buff)
          (set `local.LOCAL_FoundBuff` _array_element)
          (break)))
      (:`else`)))
  (bind _local_foundbuff (`local.LOCAL_FoundBuff`)
    (:`then`
      (`/Game/SoulslikeFramework/Data/Buffs/Logic/B_Buff.Event OnRemoved` _local_foundbuff)
      (`KismetArrayLibrary.Array_RemoveItem` (`self.ActiveBuffs`) _local_foundbuff)
      (`self.OnBuffDetected` (`local.Buff`)))
    (:`else`)))

(fn `RemoveBuffWithTag`
  (params (Tag :type "GameplayTag Structure"))
  ;[0.05098 0.05098 0.05098] Finds the first buff using the Buff tag. Removes it and stops tracking it.
  (bind _buffs (`self.GetBuffsWithTag` Tag))
  (if (`KismetArrayLibrary.Array_IsNotEmpty` _buffs)
    (bind _output (`|GetArrayItem` _buffs))
    (`/Game/SoulslikeFramework/Data/Buffs/Logic/B_Buff.Event OnRemoved` _output)
    (`KismetArrayLibrary.Array_RemoveItem` (`self.ActiveBuffs`) _output)
    (`self.OnBuffDetected` (`/Game/SoulslikeFramework/Data/Buffs/Logic/B_Buff.BuffData` _output))))