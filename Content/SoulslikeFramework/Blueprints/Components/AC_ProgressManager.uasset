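; Actor component that tracks game progress states and playtime for the Soulslike Framework.
; It seeds a gameplay-tag-to-state map from defaults, ticks playtime on a one-second timer, and restores both when the save/load component loads data.
; Serialization sends both as instanced-struct blocks under separate save tags.
; It also executes tag-switched gameplay events that grant items, currency or progress, and looks up level-up costs from a curve.
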(event `self.ReceiveBeginPlay`
  (`|ExecutionSequence`
    (:`then_0`
      ;[0.05098 0.05098 0.05098] Bind to OnDataLoaded() from Save/Load component.
      (add `/Game/SoulslikeFramework/Blueprints/Components/AC_SaveLoadManager.OnDataLoaded` (`/Game/SoulslikeFramework/Blueprints/BFL_Helper.GetSaveLoadComponent` (`GameplayStatics.GetPlayerController` 0)) (`|CreateDelegate` :!event `Event OnDataLoaded`)))
    (:`then_1`
      ;[0.05098 0.05098 0.05098] Initialize default progress data
      (bind _keys (`BlueprintMapLibrary.Map_Keys` (`self.DefaultsToProgress`)))
      (bind _values (`BlueprintMapLibrary.Map_Values` (`self.DefaultsToProgress`)))
      (for (_array_element _array_index) _keys
        (`self.SetProgress` _array_element (`|GetArrayItem` _values _array_index))))
    (:`then_2`
      ;[0.05098 0.05098 0.05098] Increase playtime timer on a 1.0 sec interval.
      (`KismetSystemLibrary.K2_SetTimerDelegate` (delegate `Event PlayTimeTimer`) 1.0 true))))

(event `Event PlayTimeTimer`
  ;[0.05098 0.05098 0.05098] Increase playtime timer on a 1.0 sec interval.
  (bind _output_get (set `self.PlayTime` (+ (`self.PlayTime`) (`KismetMathLibrary.MakeTimespan` 0 0 0 1))))
  (`self.OnPlayTimeUpdated` _output_get))

(event `Event OnDataLoaded`
  (params (LoadedData :type "/Game/SoulslikeFramework/Structures/Saving/FSaveGameInfo Structure"))
  (`|ExecutionSequence`
    (:`then_0`
      ;[0.05098 0.05098 0.05098] Retrieve Progress save data block and add them to CurrentProgress[] map of Progress Tag | EProgress.
      (bind (_success_ _returnvalue) (`/Game/SoulslikeFramework/Blueprints/BFL_Helper.GetSaveDataByTag` LoadedData (struct :`TagName` "SoulslikeFramework.Saving.Progress")))
      (if _success_
        (bind _values (`/Game/SoulslikeFramework/Blueprints/BML_StructConversion.ConvertToProgressSaveInfoStructs` _returnvalue))
        (`self.Event InitializeLoadedProgress` _values)))
    (:`then_1`
      ;[0.05098 0.05098 0.05098] Retrieve PlayTime save data block and set PlayTime timespan to loaded value.
      (bind (_success__2 _returnvalue_2) (`/Game/SoulslikeFramework/Blueprints/BFL_Helper.GetSaveDataByTag` LoadedData (struct :`TagName` "SoulslikeFramework.Saving.PlayTime")))
      (if _success__2
        (bind _value (`/Game/SoulslikeFramework/Blueprints/BML_StructConversion.ConvertToTimespanStruct` _returnvalue_2))
        (`self.Event InitializeLoadedPlayTime` _value)))))

(event `Event InitializeLoadedPlayTime`
  (params (PlayTime :type "Timespan Structure"))
  ;[0.05098 0.05098 0.05098] Called from AC_SaveLoadManager when data is loaded
  (set `self.PlayTime` PlayTime))

(event `Event InitializeLoadedProgress`
  (params (LoadedProgress :type "Array of /Game/SoulslikeFramework/Structures/Saving/FProgressSaveInfo Structure"))
  ;[0.05098 0.05098 0.05098] Called when progress data is loaded
  (for _array_element LoadedProgress
    (bind (_progresstag _progressstate) (break `/Game/SoulslikeFramework/Structures/Saving/FProgressSaveInfo` _array_element))
    (`self.SetProgress` _progresstag _progressstate)))

(fn `ExecuteGameplayEvents`
  (params (GameplayEvents :type "Array of /Game/SoulslikeFramework/Structures/Dialog/FDialogGameplayEvent Structure"))
  (locals (LOCAL_EventTag :type "GameplayTag Structure") (LOCAL_AdditionalTag :type "GameplayTag Structure") (LOCAL_Data :type "InstancedStruct Structure"))
  ;[0.05098 0.05098 0.05098] Executes a gameplay event. Feel free to extend this as you desire. The provided example below is used in the Showcase NPC's dialogs.
  (for _array_element GameplayEvents
    (bind (_eventtag _additionaltag _customdata) (break `/Game/SoulslikeFramework/Structures/Dialog/FDialogGameplayEvent` _array_element))
    (set `local.LOCAL_EventTag` _eventtag)
    (set `local.LOCAL_AdditionalTag` _additionaltag)
    (set `local.LOCAL_Data` _customdata)
    (`|SwitchGameplayTag` (`local.LOCAL_EventTag`)
      (:`SoulslikeFramework.GameplayEvents.AddItem`
        ;[0.05098 0.05098 0.05098] Add item with tag & with desired amount to inventory.
        (bind _value (`/Game/SoulslikeFramework/Blueprints/BML_StructConversion.ConvertToFInt` (`local.LOCAL_Data`))
          (:`Then`
            (`/Game/SoulslikeFramework/Blueprints/Components/AC_InventoryManager.Event AsyncAddItemByTag` (`Actor.GetComponentByClass` (`self.GetOwner`) "/Game/SoulslikeFramework/Blueprints/Components/AC_InventoryManager.AC_InventoryManager_C") (`local.LOCAL_AdditionalTag`) (`.Int_31_1635518D4B5EA126D75B9481FB7F017E` (break `/Game/SoulslikeFramework/Structures/_Misc/FInt` _value)) true))))
      (:`SoulslikeFramework.GameplayEvents.AddCurrency`
        ;[0.05098 0.05098 0.05098] Adjust currency with the desired amount.
        (bind _value_2 (`/Game/SoulslikeFramework/Blueprints/BML_StructConversion.ConvertToFInt` (`local.LOCAL_Data`))
          (:`Then`
            (`/Game/SoulslikeFramework/Blueprints/Components/AC_InventoryManager.AdjustCurrency` (`Actor.GetComponentByClass` (`self.GetOwner`) "/Game/SoulslikeFramework/Blueprints/Components/AC_InventoryManager.AC_InventoryManager_C") (`.Int_31_1635518D4B5EA126D75B9481FB7F017E` (break `/Game/SoulslikeFramework/Structures/_Misc/FInt` _value_2))))))
      (:`SoulslikeFramework.GameplayEvents.AddProgress`
        ;[0.05098 0.05098 0.05098] Set progress of the desired progress to EProgress.
        (bind _value_3 (`/Game/SoulslikeFramework/Blueprints/BML_StructConversion.ConvertToFProgress` (`local.LOCAL_Data`))
          (:`Then`
            (`self.SetProgress` (`/Game/SoulslikeFramework/Blueprints/BFL_Helper.GetLocalProgressManager`) (`local.LOCAL_AdditionalTag`) (`.Progress_2_6978876E49F83EBD70A0E286FBA704DF` (break `/Game/SoulslikeFramework/Structures/_Misc/FProgress` _value_3)))))))))

(fn `GetProgress`
  (params (ProgressTag :type "GameplayTag Structure"))
  (returns (`Found?` :type Boolean) (State :type "/Game/SoulslikeFramework/Enums/E_Progress Enum"))
  (bind (_value _returnvalue) (`BlueprintMapLibrary.Map_Find` (`self.CurrentProgress`) ProgressTag))
  ;[0.05098 0.05098 0.05098] Gets progress and its state
  (if _returnvalue
    (return true _value)
    (else
      (return false "NewEnumerator0"))))

(fn `GetRequiredCurrencyForLevel`
  (params (Level :type Integer))
  (returns (ReturnValue :type Integer))
  ;[0.05098 0.05098 0.05098] Returns currency cost for target level
  (return (`KismetMathLibrary.Round` (`CurveFloat.GetFloatValue` (`self.LevelUpCosts`) (`KismetMathLibrary.Conv_IntToDouble` Level)))))

(fn `SerializeProgressData`
  (locals (LOCAL_InstancedProgressData :type "Array of InstancedStruct Structure"))
  ;[0.05098 0.05098 0.05098] Loops through each progress entry item, creating an instanced struct for each with its tag and EProgress. This struct holds individual progress data, making it easy to save progress separately. Once all progress entries are processed, triggers a save request to AC_SaveLoadManager, sending the structured progress data for saving. Additionally, does the same for PlayTime as a separate save data block.
  (bind _keys (`BlueprintMapLibrary.Map_Keys` (`self.CurrentProgress`)))
  (bind _values (`BlueprintMapLibrary.Map_Values` (`self.CurrentProgress`)))
  (for (_array_element _array_index) _keys
    (bind _returnvalue (`BlueprintInstancedStructLibrary.MakeInstancedStruct` (make `/Game/SoulslikeFramework/Structures/Saving/FProgressSaveInfo` _array_element (`|GetArrayItem` _values _array_index))))
    (`KismetArrayLibrary.Array_Add` (`local.LOCAL_InstancedProgressData`) _returnvalue))
  (message `/Game/SoulslikeFramework/Blueprints/Interfaces/BPI_Controller.RequestUpdateSaveData` (`GameplayStatics.GetPlayerController` 0) (struct :`TagName` "SoulslikeFramework.Saving.Progress") (`local.LOCAL_InstancedProgressData`))
  (bind _returnvalue_2 (`BlueprintInstancedStructLibrary.MakeInstancedStruct` (`self.PlayTime`)))
  (message `/Game/SoulslikeFramework/Blueprints/Interfaces/BPI_Controller.RequestUpdateSaveData` (`GameplayStatics.GetPlayerController` 0) (struct :`TagName` "SoulslikeFramework.Saving.PlayTime") (`|MakeArray` _returnvalue_2)))

(fn `SetProgress`
  (params (ProgressTag :type "GameplayTag Structure") (State :type "/Game/SoulslikeFramework/Enums/E_Progress Enum" :default "NewEnumerator0"))
  (bind _currentprogress (`self.CurrentProgress`))
  ;[0.05098 0.05098 0.05098] Sets desired progress with desired state
  (`BlueprintMapLibrary.Map_Add` (`self.CurrentProgress`) ProgressTag State)
  ;[0.05098 0.05098 0.05098] Debug
  (bind _keys (`BlueprintMapLibrary.Map_Keys` _currentprogress))
  (bind _values (`BlueprintMapLibrary.Map_Values` _currentprogress))
  (for (_array_element _array_index) _keys
    (`KismetSystemLibrary.PrintText` (`|FormatText` "Progress: {prog} | State: {state}" (`BlueprintGameplayTagLibrary.GetDebugStringFromGameplayTag` _array_element) (`|GetEnumeratorNameAsString` (`|GetArrayItem` _values _array_index))) true true (struct :`R` 0.246394 :`G` 1.0 :`A` 1.0) 10.0)))