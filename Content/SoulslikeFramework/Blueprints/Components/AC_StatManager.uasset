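; Stat manager component for players and AI, owning per-stat objects, their queries and adjustments, and the player level.
; BeginPlay builds stat objects from a data table or map, then applies overrides or the player's class base stats.
; Stat updates can cascade into dependent stats through softcap ranges, using level curves or modifier calculations.
; Stats and level serialize as instanced structs for saving, and non-AI components restore them when save data loads.
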(fn `AdjustAffected`
  (params (StatTag :type "GameplayTag Structure") (ValueType :type "/Game/SoulslikeFramework/Enums/E_ValueType Enum" :default "NewEnumerator0") (Change :type "Float (double-precision)"))
  (bind _found_stat (`self.GetStat` StatTag))
  ;[0.05098 0.05098 0.05098] Function to update affected stats of a stat.
  (`/Engine/EditorBlueprintResources/StandardMacros.IsValid` _found_stat
    (:`Is Valid`
      (`/Game/SoulslikeFramework/Data/Stats/B_Stat.AdjustAffectedValue` _found_stat ValueType Change))))

(fn `AdjustAffectedStats`
  (params (Stat :type "/Game/SoulslikeFramework/Data/Stats/B_Stat Object Reference") (Change :type "Float (double-precision)") (ValueType :type "/Game/SoulslikeFramework/Enums/E_ValueType Enum" :default "NewEnumerator0"))
  (bind ((`DisplayName_45_55A184B14E56D9C63DBBD68E4B70971B` _displayname) (`DisplayAsPercent_46_96ECE4D54F594255EBEC728EA8B68917` _displayaspercent) (`CurrentValue_47_EEB1DDB64CB05B32EFEB3987C7578E44` _currentvalue)) (break `/Game/SoulslikeFramework/Structures/Stats/FStatInfo` (`/Game/SoulslikeFramework/Data/Stats/B_Stat.StatInfo` (`local.Stat`))))
  (bind _statstoaffect (break `/Game/SoulslikeFramework/Structures/Stats/FStatBehavior` (`.StatModifiers_51_437F7248490379A115E46EB53AA885B3` (break `/Game/SoulslikeFramework/Structures/Stats/FStatInfo` (`/Game/SoulslikeFramework/Data/Stats/B_Stat.StatInfo` (`local.Stat`))))))
  ;[0.05098 0.05098 0.05098] Critical function which is used to update affected stats of a stat which has recently been changed. For e.g, when B_Vigor is changed, this function will find it's affected stat(s) (B_Health, in our demo) and attempt to update it accordingly!
  (if (> (`BlueprintMapLibrary.Map_Length` _statstoaffect) 0)
    (bind _keys (`BlueprintMapLibrary.Map_Keys` _statstoaffect))
    (bind _values (`BlueprintMapLibrary.Map_Values` _statstoaffect))
    (for (_array_element _array_index) _keys
      (for _array_element_2 (`.SoftcapData_26_AF4CAD8043134AE8B54B869A29D1F5DF` (break `/Game/SoulslikeFramework/Structures/Stats/FAffectedStats` (`|GetArrayItem` _values _array_index)))
        (bind ((`FromLevel_23_910B362F47B36A93743811A1545901E7` _fromlevel) (`UntilLevel_25_B7D2BF5042CD96C0041128B8DBAFA732` _untillevel)) (break `/Game/SoulslikeFramework/Structures/Stats/FAffectedStat` _array_element_2))
        (if (and (>= _currentvalue _fromlevel) (<= _currentvalue _untillevel))
          (bind ((`AffectMaxValue?_8_77FBB64C4E23F6E7C04A46B9C432D4B7` _affectmaxvalue_) (`Modifier_5_29F8F0E54638A580CDE4C592A94F2A5A` _modifier) (`Calculation_15_BF33800E4B1FF59B8E2E99B27FE31A05` _calculation) (`ChangebyCurveOptional_18_AF4CAD8043134AE8B54B869A29D1F5DF` _changebycurveoptional)) (break `/Game/SoulslikeFramework/Structures/Stats/FAffectedStat` _array_element_2))
          (if _affectmaxvalue_
            (`/Engine/EditorBlueprintResources/StandardMacros.IsValid` _changebycurveoptional
              (:`Is Valid`
                (bind _outchange (`/Game/SoulslikeFramework/Data/Calculators/PDA_Calculations.Calculate` _calculation _modifier (`local.Change`)))
                (bind _returnvalue (select `bool` (`KismetSystemLibrary.IsValid` _changebycurveoptional) :`false` _outchange :`true` (`CurveFloat.GetFloatValue` _changebycurveoptional (`KismetMathLibrary.Conv_IntToDouble` (`self.Level`))) :!type "Float (double-precision)"))
                (`self.AdjustAffected` _array_element "NewEnumerator1" _returnvalue))
              (:`Is Not Valid`
                (`self.AdjustAffected` _array_element "NewEnumerator1" _outchange)))
            (else
              (`/Engine/EditorBlueprintResources/StandardMacros.IsValid` _changebycurveoptional
                (:`Is Valid`
                  (`self.AdjustAffected` _array_element "NewEnumerator0" _returnvalue))
                (:`Is Not Valid`
                  (`self.AdjustAffected` _array_element "NewEnumerator0" _outchange))))))))
    (return)
    (else
      (return))))

(fn `AdjustLevel`
  (params (Delta :type Integer))
  ;[0.05098 0.05098 0.05098] Adjust level and notify relevant widgets using the dispatcher.
  (if (not (`self.IsAiComponent`))
    (bind _output_get (set `self.Level` (+ (`self.Level`) Delta)))
    (`self.OnLevelUpdated` _output_get)))

(fn `AdjustStat`
  (params (StatTag :type "GameplayTag Structure") (ValueType :type "/Game/SoulslikeFramework/Enums/E_ValueType Enum" :default "NewEnumerator0") (Change :type "Float (double-precision)") (`Level Up?` :type Boolean) (`TriggerRegen?` :type Boolean))
  (bind _found_stat (`self.GetStat` StatTag))
  ;[0.05098 0.05098 0.05098] Function to update stat by its ID.
  (`/Engine/EditorBlueprintResources/StandardMacros.IsValid` _found_stat
    (:`Is Valid`
      (`/Game/SoulslikeFramework/Data/Stats/B_Stat.AdjustValue` _found_stat ValueType Change `Level Up?` `TriggerRegen?`))))

(fn `GetAllStats`
  (returns (StatObjects :type "Array of /Game/SoulslikeFramework/Data/Stats/B_Stat Object Reference") (StatClassesAndCategories :type "Map of /Game/SoulslikeFramework/Data/Stats/B_Stat Class Reference to GameplayTag Structure"))
  ;[0.05098 0.05098 0.05098] Simple getter function which will return all Stat Objects, as well as the instantiation variable (Stats map) which is necessary for initialization.
  (bind _values (`BlueprintMapLibrary.Map_Values` (`self.ActiveStats`)))
  (return _values (`self.Stats`)))

(fn `GetStat`
  (params (StatTag :type "GameplayTag Structure"))
  (returns (`Found Stat` :type "/Game/SoulslikeFramework/Data/Stats/B_Stat Object Reference") (`Stat Info` :type "/Game/SoulslikeFramework/Structures/Stats/FStatInfo Structure"))
  (bind (_value _returnvalue) (`BlueprintMapLibrary.Map_Find` (`self.ActiveStats`) StatTag))
  ;[0.05098 0.05098 0.05098] Simple getter function to get stat object and stat info by its ID.
  (if _returnvalue
    (return _value (`/Game/SoulslikeFramework/Data/Stats/B_Stat.StatInfo` _value))
    (else
      (return null))))

(fn `GetStatsForCategory`
  (params (StatCategory :type "GameplayTag Structure"))
  (returns (Stats :type "GameplayTagContainer Structure"))
  (locals (LOCAL_Stats :type "Array of GameplayTag Structure") (LOCAL_StatsContainer :type "GameplayTagContainer Structure"))
  ;[0.05098 0.05098 0.05098] Returns all stat tags that are under the specified Stat Category Tag.
  (bind _keys (`BlueprintMapLibrary.Map_Keys` (`self.Stats`)))
  (bind _values (`BlueprintMapLibrary.Map_Values` (`self.Stats`)))
  (for (_array_element _array_index) _values
    (if (== _array_element (`local.StatCategory`))
      (`BlueprintGameplayTagLibrary.AddGameplayTag` (`local.LOCAL_StatsContainer`) (`.Tag_39_84F9579F432E05BBC375FD8FCBBE2158` (break `/Game/SoulslikeFramework/Structures/Stats/FStatInfo` (defaults `Object` (`|GetArrayItem` _keys _array_index)))))))
  (return (`local.LOCAL_StatsContainer`)))

(fn `InitializeLoadedStats`
  (params (LoadedStats :type "Array of /Game/SoulslikeFramework/Structures/Stats/FStatInfo Structure"))
  ;[0.05098 0.05098 0.05098] Updates the stat info struct of loaded stats.
  (if (not (`self.IsAiComponent`))
    (for _array_element (`local.LoadedStats`)
      (`/Game/SoulslikeFramework/Data/Stats/B_Stat.UpdateStatInfo` (`BlueprintMapLibrary.Map_Find` (`self.ActiveStats`) (`.Tag_39_84F9579F432E05BBC375FD8FCBBE2158` (break `/Game/SoulslikeFramework/Structures/Stats/FStatInfo` _array_element))) _array_element))
    (return)))

(fn `IsStatMoreThan`
  (params (StatTag :type "GameplayTag Structure") (Threshold :type "Float (double-precision)"))
  (returns (ReturnValue :type Boolean))
  ;[0.05098 0.05098 0.05098] Function which checks if the current value of target stat (by tag) is > Threshold
  (return (> (`.CurrentValue_47_EEB1DDB64CB05B32EFEB3987C7578E44` (break `/Game/SoulslikeFramework/Structures/Stats/FStatInfo` (`.Stat Info` (`self.GetStat` StatTag)))) (`local.Threshold`))))

(fn `ResetStat`
  (params (StatTag :type "GameplayTag Structure"))
  (bind (_found_stat _stat_info) (`self.GetStat` StatTag))
  ;[0.05098 0.05098 0.05098] Reset's target stat's current value to its max value. Used when resting.
  (`/Game/SoulslikeFramework/Data/Stats/B_Stat.AdjustValue` _found_stat "NewEnumerator0" (- (`/Game/SoulslikeFramework/Blueprints/BFL_Helper.GetStatMaxValue` _stat_info) (`/Game/SoulslikeFramework/Blueprints/BFL_Helper.GetStatCurrentValue` _stat_info)) false false))

(fn `SerializeStatsData`
  (locals (LOCAL_StatsToSave :type "Array of /Game/SoulslikeFramework/Structures/Stats/FStatInfo Structure") (LOCAL_InstancedStats :type "Array of InstancedStruct Structure"))
  ;[0.05098 0.05098 0.05098] Method which loops through all stat objects, retrieves their info and makes an array of Instanced Structs using the data which is then sent to AC_SaveLoadManager for saving. Does the same for player level.
  (`KismetArrayLibrary.Array_Clear` (`local.LOCAL_StatsToSave`))
  (for _array_element (`self.GetAllStats`)
    (bind _statinfo (`/Game/SoulslikeFramework/Data/Stats/B_Stat.StatInfo` _array_element))
    (`KismetArrayLibrary.Array_AddUnique` (`local.LOCAL_StatsToSave`) _statinfo)
    (bind _returnvalue (`BlueprintInstancedStructLibrary.MakeInstancedStruct` _statinfo))
    (`KismetArrayLibrary.Array_Add` (`local.LOCAL_InstancedStats`) _returnvalue))
  (message `/Game/SoulslikeFramework/Blueprints/Interfaces/BPI_Controller.RequestUpdateSaveData` (`GameplayStatics.GetPlayerController` 0) (struct :`TagName` "SoulslikeFramework.Saving.Stats") (`local.LOCAL_InstancedStats`))
  ;;[0.05098 0.05098 0.05098] Save level separately
  (bind _returnvalue_2 (`BlueprintInstancedStructLibrary.MakeInstancedStruct` (make `/Game/SoulslikeFramework/Structures/_Misc/FInt` (`self.Level`))))
  (message `/Game/SoulslikeFramework/Blueprints/Interfaces/BPI_Controller.RequestUpdateSaveData` (`GameplayStatics.GetPlayerController` 0) (struct :`TagName` "SoulslikeFramework.Saving.PlayerLevel") (`|MakeArray` _returnvalue_2)))

(fn `ToggleRegenForStat`
  (params (StatTag :type "GameplayTag Structure") (`Stop?` :type Boolean))
  (bind (_value _returnvalue) (`BlueprintMapLibrary.Map_Find` (`self.ActiveStats`) StatTag))
  (if _returnvalue
    (`/Game/SoulslikeFramework/Data/Stats/B_Stat.Event ToggleStatRegen` _value (`local.Stop?`))))