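; Character component that drives soulslike ladder climbing, including entering from the top, looping up or down and climbing out at the top or bottom.
; Move input plays async-loaded montages from a ladder animset, gated by an anim state that notifies reset, while sprint scales their play rate.
; Setters for ground, top and climbing status trigger transitions, switch movement between Flying and Walking and flag AC_ActionManager as on-ladder to block actions.
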(event `EnhancedInput|/Game/SoulslikeFramework/Input/Actions/IA_Sprint_Dodge`
  (params (ActionValue :type Boolean) (ElapsedSeconds :type "Float (double-precision)") (TriggeredSeconds :type "Float (double-precision)") (InputAction :type "InputAction Object Reference" :default "/Game/SoulslikeFramework/Input/Actions/IA_Sprint_Dodge.IA_Sprint_Dodge"))
  ;[0.05098 0.05098 0.05098] Adjust climbing montages' play rates if trying to sprint while climbing up/down.
  (:`Started`
    (set `self.ClimbFast?` true)
    (bind (_climb_up _climb_down) (`self.TryLoadClimbMontages` :!label _label))
    (bind _ascharacter (cast `Character` (`self.GetOwner`)))
    (bind _returnvalue (`SkeletalMeshComponent.GetAnimInstance` (`Character.Mesh` _ascharacter)))
    (bind _returnvalue_2 (`AnimInstance.GetCurrentActiveMontage` _returnvalue))
    (if (or (== _returnvalue_2 _climb_up) (== _returnvalue_2 _climb_down))
      (`AnimInstance.Montage_SetPlayRate` _returnvalue _returnvalue_2 (`KismetMathLibrary.SelectFloat` (`self.ClimbSprintMultiplier`) 1.0 (`self.ClimbFast?`)))))
  (:`Completed`
    (set `self.ClimbFast?` false)
    (goto _label)))

(event `EnhancedInput|/Game/SoulslikeFramework/Input/Actions/IA_Move`
  (params (ActionValue :type "Vector2D Structure") (ElapsedSeconds :type "Float (double-precision)") (TriggeredSeconds :type "Float (double-precision)") (InputAction :type "InputAction Object Reference" :default "/Game/SoulslikeFramework/Input/Actions/IA_Move.IA_Move"))
  (bind (_x _y) (`KismetMathLibrary.BreakVector2D` ActionValue))
  (:`Triggered`
    ;[0.05098 0.05098 0.05098] Ensure that we're not playing any montage
    (switch `/Game/SoulslikeFramework/Enums/E_LadderClimbState` (`self.ClimbAnimState`)
      (:`NewEnumerator0`
        ;[0.05098 0.05098 0.05098] Are we climbing? & are we on the ground?
        (if (`self.IsClimbing`)
          (if (and (`self.IsOnGround`) (`self.IsClimbing`) (< _y 0.0))
            (`self.SetIsClimbing` false)
            ;[0.05098 0.05098 0.05098] Get out of ladder at the bottom
            (bind _object (`|LoadAsset` (`/Game/SoulslikeFramework/Data/_AnimationData/PDA_LadderAnimData.ClimbDown` (`self.LadderAnimset`)))
              (:`Completed`
                (bind _asanim_montage (cast `AnimMontage` _object))
                (bind _ascharacter (cast `Character` (`self.GetOwner`)))
                (`AnimInstance.Montage_Stop` (`SkeletalMeshComponent.GetAnimInstance` (`Character.Mesh` _ascharacter)) 0.25 _asanim_montage)
                (set `self.ClimbAnimState` "NewEnumerator0")))
            (elif (`self.IsOrientedToLadder`)
              ;[0.05098 0.05098 0.05098] Climb up or down based on input.
              (switch `/Game/SoulslikeFramework/Enums/E_LadderClimbState` (`self.ClimbAnimState`)
                (:`NewEnumerator0`
                  (set `self.ClimbAnimState` "NewEnumerator1")
                  (bind (_climb_up _climb_down) (`self.TryLoadClimbMontages`))
                  (bind _ascharacter_2 (cast `Character` (`self.GetOwner`)))
                  (bind _mesh (`Character.Mesh` _ascharacter_2)
                    (:`then`
                      (bind _notifyname (`|PlayMontage` _mesh (select `bool` (and (`self.IsClimbing`) (not (`self.IsOnGround`)) (< _y 0.0)) :`false` _climb_up :`true` _climb_down) (`KismetMathLibrary.SelectFloat` (`self.ClimbSprintMultiplier`) 1.0 (`self.ClimbFast?`)))
                        (:`OnNotifyBegin`
                          (if (== _notifyname "Loop_End")
                            (set `self.ClimbAnimState` "NewEnumerator0")))))
                    (:`else`)))))))))))

(event `Event OnClimbOut`
  ;[0.05098 0.05098 0.05098] Handles climbing out of the ladder. Will play relative montage and adjust anim state
  (bind _object (`|LoadAsset` (`/Game/SoulslikeFramework/Data/_AnimationData/PDA_LadderAnimData.ClimbOutAtTop` (`self.LadderAnimset`)))
    (:`Completed`
      (bind _asanim_montage (cast `AnimMontage` _object))
      (bind _ascharacter (cast `Character` (`self.GetOwner`)))
      (bind _mesh (`Character.Mesh` _ascharacter)
        (:`then`
          (`|PlayMontage` _mesh _asanim_montage
            (:`then`
              (set `self.ClimbAnimState` "NewEnumerator2"))
            (:`OnCompleted`
              (set `self.ClimbAnimState` "NewEnumerator0")
              (`self.SetIsClimbing` false)
              (set `self.IsOrientedToLadder` false))))
        (:`else`)))))

(event `Event OnClimbDownFromTop`
  ;[0.05098 0.05098 0.05098] Handles climbing into the ladder from top. Will play relative montage and adjust anim state. The reason we use OnNotifyBegin and not OnComplete is because the montage does not blend out automatically, thus OnCompleted won't trigger.
  (bind _object (`|LoadAsset` (`/Game/SoulslikeFramework/Data/_AnimationData/PDA_LadderAnimData.ClimbInFromTop` (`self.LadderAnimset`)))
    (:`Completed`
      (bind _asanim_montage (cast `AnimMontage` _object))
      (bind _ascharacter (cast `Character` (`self.GetOwner`)))
      (bind _mesh (`Character.Mesh` _ascharacter)
        (:`then`
          (`|PlayMontage` _mesh _asanim_montage
            (:`then`
              (set `self.ClimbAnimState` "NewEnumerator3")
              (`self.SetIsClimbing` true))
            (:`OnNotifyBegin`
              (set `self.ClimbAnimState` "NewEnumerator0")
              ;[0.05098 0.05098 0.05098] After top-down climb is finished, play climb down once to avoid Top Collision issues.
              (bind (_climb_up _climb_down) (`self.TryLoadClimbMontages`))
              (bind _ascharacter_2 (cast `Character` (`self.GetOwner`)))
              (bind _mesh_2 (`Character.Mesh` _ascharacter_2)
                (:`then`
                  (bind _notifyname (`|PlayMontage` _mesh_2 _climb_down)
                    (:`then`
                      (set `self.ClimbAnimState` "NewEnumerator1"))
                    (:`OnNotifyBegin`
                      (if (== _notifyname "Loop_End")
                        (set `self.ClimbAnimState` "NewEnumerator0")))))
                (:`else`)))))
        (:`else`)))))

(fn `SetCurrentLadder`
  (params (CurrentLadder :type "/Game/SoulslikeFramework/Blueprints/_WorldActors/Interactables/B_Ladder Object Reference"))
  ;[0.05098 0.05098 0.05098] Sets current ladder to target ladder.
  (set `self.CurrentLadder` CurrentLadder))

(fn `SetIsClimbing`
  (params (IsClimbing :type Boolean))
  (bind _returnvalue (`Actor.GetComponentByClass` (`self.GetOwner`) "/Script/Engine.CharacterMovementComponent"))
  (bind _returnvalue_2 (`Actor.GetComponentByClass` (`self.GetOwner`) "/Game/SoulslikeFramework/Blueprints/Components/AC_ActionManager.AC_ActionManager_C"))
  ;[0.05098 0.05098 0.05098] If true, set movement mode to flying, disable orientation, stop movement, adjust flying decelaration and set IsOnLadder inside AC_ActionManager so actions can't be triggered
  (bind _output_get (set `self.IsClimbing` IsClimbing))
  (if _output_get
    (`CharacterMovementComponent.SetMovementMode` _returnvalue "MOVE_Flying" 0)
    (set `CharacterMovementComponent.bOrientRotationToMovement` false _returnvalue)
    (`MovementComponent.StopMovementImmediately` _returnvalue)
    (set `CharacterMovementComponent.BrakingDecelerationFlying` 5000.0 _returnvalue)
    (`/Engine/EditorBlueprintResources/StandardMacros.IsValid` _returnvalue_2
      (:`Is Valid`
        (set `/Game/SoulslikeFramework/Blueprints/Components/AC_ActionManager.IsOnLadder` true _returnvalue_2)))
    (else
      (set `CharacterMovementComponent.bOrientRotationToMovement` true _returnvalue)
      (`CharacterMovementComponent.SetMovementMode` _returnvalue "MOVE_Walking" 0)
      (`/Engine/EditorBlueprintResources/StandardMacros.IsValid` _returnvalue_2
        (:`Is Valid`
          (set `/Game/SoulslikeFramework/Blueprints/Components/AC_ActionManager.IsOnLadder` false _returnvalue_2))))))

(fn `SetIsClimbingDownFromTop`
  (params (IsClimbingDownFromTop :type Boolean))
  ;[0.05098 0.05098 0.05098] If we're NOT climbing, play related ClimbDownFromTop montage.
  (bind _output_get (set `self.IsClimbingDownFromTop` IsClimbingDownFromTop))
  (if (and _output_get (not (`self.IsClimbing`)))
    (`self.Event OnClimbDownFromTop`)))

(fn `SetIsClimbingOffTop`
  (params (IsClimbingOffTop :type Boolean))
  (bind _output_get (set `self.IsClimbingOffTop` IsClimbingOffTop))
  (if _output_get
    ;[0.05098 0.05098 0.05098] Reset anim state and play related climb out montage.
    (if (`self.IsClimbing`)
      (switch `/Game/SoulslikeFramework/Enums/E_LadderClimbState` (`self.ClimbAnimState`)
        (:`NewEnumerator0`
          _)
        (:`NewEnumerator1`
          _))
      (set `self.ClimbAnimState` "NewEnumerator0")
      (`self.Event OnClimbOut`))
    (else
      ;[0.05098 0.05098 0.05098] Only switch to Walking mode if we're NOT climbing and are oriented to the ladder
      (if (and (not (`self.IsClimbing`)) (`self.IsOrientedToLadder`))
        (`CharacterMovementComponent.SetMovementMode` (`Actor.GetComponentByClass` (`self.GetOwner`) "/Script/Engine.CharacterMovementComponent") "MOVE_Walking" 0)))))

(fn `SetIsOnGround`
  (params (IsOnGround :type Boolean))
  (bind _returnvalue (`Actor.GetComponentByClass` (`self.GetOwner`) "/Script/Engine.CharacterMovementComponent"))
  ;[0.05098 0.05098 0.05098] If IsOnGround is false, we'll check if we're NOT climbing. If not, we'll adjust movement modes accordingly.
  (bind _output_get (set `self.IsOnGround` IsOnGround))
  (if _output_get
    _
    (elif (`self.IsClimbing`)
      _
      (elif (`self.IsOrientedToLadder`)
        (`CharacterMovementComponent.SetMovementMode` _returnvalue "MOVE_Walking" 0)
        (set `self.IsOrientedToLadder` false)
        (elif (`self.IsClimbingDownFromTop`)
          (`CharacterMovementComponent.SetMovementMode` _returnvalue "MOVE_Walking" 0))))))