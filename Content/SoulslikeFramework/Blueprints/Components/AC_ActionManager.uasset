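; Soulslike character component that runs gameplay-tagged actions and tracks movement states such as sprinting, crouching and resting.
; On BeginPlay it merges an optional DataTable into its action map, recursively async-loads each class and constructs action objects, which PerformAction executes unless on a ladder.
; Movement input becomes an eight-way or idle direction, relayed via server and multicast events, for selecting dodge montages.
; A looping timer drains sprint stamina while moving and triggers StopSprinting when empty.
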(event `self.ReceiveBeginPlay`
  (`self.OverrideTable`
    (:`then`
      (bind _outrownames (`DataTableFunctionLibrary.GetDataTableRowNames` (`self.OverrideTable`)))
      (for _array_element _outrownames
        (bind _returnvalue (`|GetDataTableRow` (`self.OverrideTable`) _array_element)
          (:`then`
            (bind (_tag _actionasset) (break `/Game/SoulslikeFramework/Structures/Actions/FActionsData` _returnvalue))
            (`BlueprintMapLibrary.Map_Add` (`self.Actions`) _tag _actionasset)))))
    (:`else`
      _))
  (if (not (`BlueprintMapLibrary.Map_IsEmpty` (`self.Actions`)))
    (bind _keys (`BlueprintMapLibrary.Map_Keys` (`self.Actions`)))
    (set `self.ActionTagsCache` _keys)
    (bind _values (`BlueprintMapLibrary.Map_Values` (`self.Actions`)))
    (set `self.ActionAssetsCache` _values)
    (`self.Event RecursiveLoadActions`)
    (else
      (`KismetSystemLibrary.PrintText` "AC_ActionManager: Could not find any actions. Ensure that you have selected your actions or have a valid OverrideTable." true true (struct :`R` 0.359375 :`G` 0.005616 :`B` 0.005616 :`A` 1.0) 10.0))))

(event `Event RecursiveLoadActions`
  (bind _output (`|GetArrayItem` (`self.ActionAssetsCache`)))
  (if (not (or (`KismetArrayLibrary.Array_IsEmpty` (`self.ActionAssetsCache`)) (`KismetArrayLibrary.Array_IsEmpty` (`self.ActionTagsCache`))))
    (bind _actionclass (`/Game/SoulslikeFramework/Data/Actions/ActionData/PDA_Action.ActionClass` _output)
      (:`then`
        (bind _class (`|LoadAssetClass` _actionclass)
          (:`Completed`
            (bind _asaction_object (castclass `/Game/SoulslikeFramework/Data/Actions/ActionLogic/B_Action` _class))
            (bind _returnvalue (`|GenericCreateObject` _asaction_object _output (`self.GetOwner`)))
            (`BlueprintMapLibrary.Map_Add` (`self.AvailableActions`) (`|GetArrayItem` (`self.ActionTagsCache`)) _returnvalue)
            (`KismetArrayLibrary.Array_Remove` (`self.ActionAssetsCache`))
            (`KismetArrayLibrary.Array_Remove` (`self.ActionTagsCache`))
            (`self.Event RecursiveLoadActions`))))
      (:`else`))))

(event `Event StartStaminaLoss`
  (params (Tick :type "Float (single-precision)") (Change :type "Float (double-precision)"))
  (bind _returnvalue (`KismetSystemLibrary.K2_SetTimerDelegate` (delegate `Event ReduceStamina`) Tick true))
  (set `self.StaminaLossTimer` _returnvalue))

(event `Event ReduceStamina`
  (bind _statmanager (`self.GetStatManager`))
  (`|ExecutionSequence`
    (:`then_0`
      (`/Engine/EditorBlueprintResources/StandardMacros.IsValid` (`self.GetStatManager`)
        (:`Is Valid`
          (if (`/Game/SoulslikeFramework/Blueprints/BFL_Helper.GetIsMoving2D?` (`Actor.GetVelocity` (`self.GetOwner`)) 1.0)
            (`/Game/SoulslikeFramework/Blueprints/Components/AC_StatManager.AdjustStat` (`self.GetStatManager`) (struct :`TagName` "SoulslikeFramework.Stat.Secondary.Stamina") "NewEnumerator0" (stale `Event StartStaminaLoss` Change) false false)))))
    (:`then_1`
      (`/Engine/EditorBlueprintResources/StandardMacros.IsValid` _statmanager
        (:`Is Valid`
          (bind _returnvalue (`/Game/SoulslikeFramework/Blueprints/Components/AC_StatManager.IsStatMoreThan` _statmanager (struct :`TagName` "SoulslikeFramework.Stat.Secondary.Stamina") 0.0))
          (if _returnvalue
            (`/Game/SoulslikeFramework/Data/Stats/B_Stat.Event ToggleStatRegen` (`/Game/SoulslikeFramework/Blueprints/Components/AC_StatManager.GetStat` (`self.GetStatManager`) (struct :`TagName` "SoulslikeFramework.Stat.Secondary.Stamina")) true)
            (else
              (`self.Event PerformAction` (struct :`TagName` "SoulslikeFramework.Action.StopSprinting")))))))))

(event `Event StopStaminaLoss`
  (bind _statmanager (`self.GetStatManager`))
  (if (`KismetSystemLibrary.K2_IsValidTimerHandle` (`self.StaminaLossTimer`))
    (`KismetSystemLibrary.K2_ClearAndInvalidateTimerHandle` (`self.StaminaLossTimer`))
    (`/Engine/EditorBlueprintResources/StandardMacros.IsValid` _statmanager :!label _label
      (:`Is Valid`
        (`/Game/SoulslikeFramework/Data/Stats/B_Stat.Event ToggleStatRegen` (`/Game/SoulslikeFramework/Blueprints/Components/AC_StatManager.GetStat` _statmanager (struct :`TagName` "SoulslikeFramework.Stat.Secondary.Stamina")) false)))))

(event `Event StartStaminaRegen`
  (goto _label))

(event `Event PerformAction`
  (params (ActionTag :type "GameplayTag Structure"))
  (bind (_value _returnvalue) (`BlueprintMapLibrary.Map_Find` (`self.AvailableActions`) ActionTag))
  ;[0.05098 0.05098 0.05098] When an action is performed, will try to find its relevant instance and execute it. If player is on a ladder, all actions are disregarded.
  (if (not (`/Game/SoulslikeFramework/Blueprints/Components/AC_ActionManager.IsOnLadder` (`Actor.GetComponentByClass` (`self.GetOwner`) "AC_ActionManager_C")))
    (if _returnvalue
      (`/Engine/EditorBlueprintResources/StandardMacros.IsValid` _value
        (:`Is Valid`
          (`/Game/SoulslikeFramework/Data/Actions/ActionLogic/B_Action.ExecuteAction` _value))))))

(event `SRV_SetDirection`
  (params (MovementDirection :type "/Game/SoulslikeFramework/Enums/E_Direction Enum" :default "NewEnumerator8"))
  ;[0.05098 0.05098 0.05098] Triggered from B_Soulslike_Character on a 0.1 sec timer. This data allows the component to keep track of player's movement vector length & direction
  (`self.MC_SetDirection` MovementDirection))

(event `MC_SetDirection`
  (params (MovementDirection :type "/Game/SoulslikeFramework/Enums/E_Direction Enum" :default "NewEnumerator8"))
  ;[0.05098 0.05098 0.05098] Triggered from B_Soulslike_Character on a 0.1 sec timer. This data allows the component to keep track of player's movement vector length & direction
  (set `self.MovementDirection` MovementDirection))

(fn `GetCombatManager`
  (returns (CombatManager :type "/Game/SoulslikeFramework/Blueprints/Components/AC_CombatManager Object Reference"))
  ;[0.05098 0.05098 0.05098] AC_CombatManager getter. Component owner needs to have the component.
  (return (`Actor.GetComponentByClass` (`self.GetOwner`) "/Game/SoulslikeFramework/Blueprints/Components/AC_CombatManager.AC_CombatManager_C")))

(fn `GetDirectionalDodge`
  (params (MontageData :type "/Game/SoulslikeFramework/Structures/Animation/FDodgeMontages Structure"))
  (returns (Montage :type "AnimMontage Object Reference"))
  ;[0.05098 0.05098 0.05098] Picks dodge montage according to player's current movement direction.
  (switch `/Game/SoulslikeFramework/Enums/E_Direction` (`self.MovementDirection`)
    (:`NewEnumerator8`
      (return (`.Backstep_39_445171EA492D2774EC7E05B1573B0D28` (break `/Game/SoulslikeFramework/Structures/Animation/FDodgeMontages` (`local.MontageData`)))))
    (:`NewEnumerator0`
      (return (`.Forward_31_D52898724986107771E21081C6388DEC` (break `/Game/SoulslikeFramework/Structures/Animation/FDodgeMontages` (`local.MontageData`)))))
    (:`NewEnumerator1`
      (return (`.ForwardLeft_32_0B7FD73045F86899A2831F9149CE8E53` (break `/Game/SoulslikeFramework/Structures/Animation/FDodgeMontages` (`local.MontageData`)))))
    (:`NewEnumerator2`
      (return (`.ForwardRight_33_C039E9B3414AAAD5A6822EA9328D8319` (break `/Game/SoulslikeFramework/Structures/Animation/FDodgeMontages` (`local.MontageData`)))))
    (:`NewEnumerator3`
      (return (`.Left_34_21CB04164886F55C395327B3C30394F4` (break `/Game/SoulslikeFramework/Structures/Animation/FDodgeMontages` (`local.MontageData`)))))
    (:`NewEnumerator4`
      (return (`.Right_35_772282F84C047ECFFB53D98D91E868F8` (break `/Game/SoulslikeFramework/Structures/Animation/FDodgeMontages` (`local.MontageData`)))))
    (:`NewEnumerator5`
      (return (`.Backward_36_8617411F4CC086A9DD42818F5CDF26A7` (break `/Game/SoulslikeFramework/Structures/Animation/FDodgeMontages` (`local.MontageData`)))))
    (:`NewEnumerator6`
      (return (`.BackwardLeft_37_DED58B4D41A6B0CDBEF5DF82BFC7FCF0` (break `/Game/SoulslikeFramework/Structures/Animation/FDodgeMontages` (`local.MontageData`)))))
    (:`NewEnumerator7`
      (return (`.BackwardRight_38_53FC3E5740D85040BD7A8CB268C8ABBB` (break `/Game/SoulslikeFramework/Structures/Animation/FDodgeMontages` (`local.MontageData`)))))))

(fn `GetInteractionManager`
  (returns (InteractionManager :type "/Game/SoulslikeFramework/Blueprints/Components/AC_InteractionManager Object Reference"))
  ;[0.05098 0.05098 0.05098] AC_InteractionManager getter. Component owner needs to have the component.
  (return (`Actor.GetComponentByClass` (`self.GetOwner`) "/Game/SoulslikeFramework/Blueprints/Components/AC_InteractionManager.AC_InteractionManager_C")))

(fn `GetIsCrouched`
  (returns (IsCrouched :type Boolean))
  ;[0.05098 0.05098 0.05098] Simple bIsCrouched getter (used in ABP)
  (return (`self.IsCrouched`)))

(fn `GetStatManager`
  (returns (StatManager :type "/Game/SoulslikeFramework/Blueprints/Components/AC_StatManager Object Reference"))
  ;[0.05098 0.05098 0.05098] AC_StatManager getter. Component owner needs to have the component.
  (return (`Actor.GetComponentByClass` (`self.GetOwner`) "/Game/SoulslikeFramework/Blueprints/Components/AC_StatManager.AC_StatManager_C")))

(fn `SetIsResting`
  (params (Value :type Boolean))
  ;[0.05098 0.05098 0.05098] Set resting state
  (set `self.IsResting` Value))

(fn `SetIsSprinting`
  (params (Value :type Boolean))
  ;[0.05098 0.05098 0.05098] Set resting state
  (set `self.IsSprinting` Value))

(fn `SetMoveDir`
  (params (IA_Move :type "Vector2D Structure"))
  (locals (LOCAL_Degrees :type "Float (double-precision)" :default 0.0))
  (bind _movementvector (`self.MovementVector`))
  (bind _local_degrees (`local.LOCAL_Degrees`))
  (bind (_x _y) (`KismetMathLibrary.BreakVector2D` _movementvector))
  ;[0.05098 0.05098 0.05098] Function used for setting EMovementDirection which is responsible for selecting dodge montages.
  (set `self.MovementVector` IA_Move)
  (if (not (<= (`KismetMathLibrary.VSize2D` _movementvector) 0.1))
    (set `local.LOCAL_Degrees` (`KismetMathLibrary.DegAtan2` _y _x))
    (`|ExecutionSequence`
      (:`then_0`
        (if (`KismetMathLibrary.InRange_FloatFloat` (`local.LOCAL_Degrees`) 80.0 100.0)
          (`self.SRV_SetDirection` "NewEnumerator0")))
      (:`then_1`
        (if (`KismetMathLibrary.InRange_FloatFloat` (`local.LOCAL_Degrees`) 125.0 145.0)
          (`self.SRV_SetDirection` "NewEnumerator1")))
      (:`then_2`
        (if (`KismetMathLibrary.InRange_FloatFloat` (`local.LOCAL_Degrees`) 35.0 55.0)
          (`self.SRV_SetDirection` "NewEnumerator2")))
      (:`then_3`
        (if (`KismetMathLibrary.InRange_FloatFloat` (`local.LOCAL_Degrees`) -100.0 -80.0)
          (`self.SRV_SetDirection` "NewEnumerator5")))
      (:`then_4`
        (if (`KismetMathLibrary.InRange_FloatFloat` (`local.LOCAL_Degrees`) -145.0 -125.0)
          (`self.SRV_SetDirection` "NewEnumerator6")))
      (:`then_5`
        (if (`KismetMathLibrary.InRange_FloatFloat` (`local.LOCAL_Degrees`) -55.0 -35.0)
          (`self.SRV_SetDirection` "NewEnumerator7")))
      (:`then_6`
        (if (`KismetMathLibrary.InRange_FloatFloat` (`local.LOCAL_Degrees`) -20.0 20.0)
          (`self.SRV_SetDirection` "NewEnumerator4")))
      (:`then_7`
        (if (or (>= _local_degrees 170.0) (<= _local_degrees -170.0))
          (`self.SRV_SetDirection` "NewEnumerator3"))))
    (else
      (`self.SRV_SetDirection` "NewEnumerator8"))))

(fn `ToggleCrouch`
  ;[0.05098 0.05098 0.05098] Toggles bIsCrouching and requests speed update to Parent Character class.
  (bind _output_get (set `self.IsCrouched` (not (`self.IsCrouched`))))
  (message `/Game/SoulslikeFramework/Blueprints/Interfaces/BPI_GenericCharacter.SetMovementMode` (`self.GetOwner`) (select `bool` _output_get :`false` "NewEnumerator1" :`true` "NewEnumerator0" :!type "/Game/SoulslikeFramework/Enums/E_MovementType Enum")))