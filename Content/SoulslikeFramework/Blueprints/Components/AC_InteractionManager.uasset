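; Player component of the Soulslike Framework that handles interactable detection, target lock-on and resting at campfire-style resting points.
; Tick sphere-traces ahead of the owner and notifies the nearest interactable through BPI_Interactable.
; Lock-on toggles, picking the nearest tag-matched, living target from a camera-direction trace, with a timer releasing it beyond range.
; Resting binds to the resting point's callbacks to drive HUD fades, camera blends and input, then replenishes items and stats on exit.
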(fn `CheckTargetDistance`
  ;[0.05098 0.05098 0.05098] Compare distance to target with MaxTargetLockDistance. If exceeded, remove lock on.
  (bind _lockedontarget (`self.LockedOnTarget`)
    (:`then`
      (if (> (`Actor.GetDistanceTo` _lockedontarget (`self.GetOwner`)) (`self.MaxTargetLockDistance`))
        (`self.ResetLockOn`)))
    (:`else`)))

(fn `IsTargetLocked?`
  (returns (ReturnValue :type Boolean))
  ;[0.05098 0.05098 0.05098] Returns bTargetLocked
  (return (`self.TargetLocked`)))

(fn `LockOnTarget`
  (params (LockOnTarget :type "Actor Object Reference") (`RotateTowards?` :type Boolean :default true))
  ;[0.05098 0.05098 0.05098] Locks onto a specified target, which must inherit from B_BaseCharacter. Attempts to cast the target to B_BaseCharacter; if successful, sets the target as Locked on Target and toggles the target's lock-on icon visibility. Updates the Target Locked status and triggers the On Target Locked event for further interaction handling. This ensures the target is compatible with lock-on functionality and provides visual feedback.
  (`/Engine/EditorBlueprintResources/StandardMacros.IsValid` LockOnTarget
    (:`Is Valid`
      (if (not (`/Game/SoulslikeFramework/Blueprints/BFL_Helper.IsEnemyDead?` LockOnTarget))
        (set `self.LockedOnTarget` (`local.LockOnTarget`))
        (message `/Game/SoulslikeFramework/Blueprints/Interfaces/BPI_GenericCharacter.ToggleLockonWidget` (`local.LockOnTarget`) true)
        (bind _component (message `/Game/SoulslikeFramework/Blueprints/Interfaces/BPI_GenericCharacter.GetLockonComponent` (`local.LockOnTarget`)))
        (set `self.LockedOnComponent` _component)
        (set `self.TargetLocked` true)
        (message `/Game/SoulslikeFramework/Blueprints/Interfaces/BPI_Player.OnTargetLocked` (`self.GetOwner`) true (`local.RotateTowards?`))
        (bind _returnvalue (`KismetSystemLibrary.K2_SetTimer` null "CheckTargetDistance" 1.0 true))
        (set `self.TargetLockDistanceTimer` _returnvalue)
        (else
          (message `/Game/SoulslikeFramework/Blueprints/Interfaces/BPI_Player.ResetCameraView` (`self.GetOwner`) 4.0 :!label _label))))
    (:`Is Not Valid`
      (goto _label))))

(fn `RemoveFromNearbyInteractables`
  (params (Item :type "Actor Object Reference (by ref)"))
  ;[0.05098 0.05098 0.05098] Removes item from nearby interactables
  (`KismetArrayLibrary.Array_RemoveItem` (`self.NearbyInteractables`) Item))

(fn `ResetLockOn`
  ;[0.05098 0.05098 0.05098] Resets the current lock-on target. Clears the Target Locked status and toggles the lock-on icon visibility to off. Resets the Locked on Target reference, effectively removing the player’s lock-on focus.
  (set `self.TargetLocked` false)
  (message `/Game/SoulslikeFramework/Blueprints/Interfaces/BPI_Player.OnTargetLocked` (`self.GetOwner`) false true)
  (bind _lockedontarget (`self.LockedOnTarget`)
    (:`then`
      (message `/Game/SoulslikeFramework/Blueprints/Interfaces/BPI_GenericCharacter.ToggleLockonWidget` _lockedontarget false)
      (set `self.LockedOnTarget` null)
      (set `self.LockedOnComponent` null)
      (`KismetSystemLibrary.K2_ClearAndInvalidateTimerHandle` (`self.TargetLockDistanceTimer`)))
    (:`else`)))

(fn `TargetLockTrace`
  (returns (OutHits :type "Array of HitResult Structure"))
  (bind _returnvalue (`self.GetOwner`))
  (bind _returnvalue_2 (`SceneComponent.K2_GetComponentLocation` (`Actor.GetComponentByClass` _returnvalue "/Script/Engine.CapsuleComponent")))
  ;[0.05098 0.05098 0.05098] Executes a sphere trace for locking onto potential targets. Determines the trace start and end points based on the player’s location and forward vector, scaled by the specified trace distance and radius. Filters the trace by specified object types and ignores the player. The results (Out Hits) are returned, identifying possible lock-on targets within range
  (bind _outhits (`KismetSystemLibrary.SphereTraceMultiForObjects` _returnvalue_2 (+ _returnvalue_2 (* (`SceneComponent.GetForwardVector` (`Actor.GetComponentByClass` _returnvalue "/Script/Engine.CameraComponent")) (`self.TargetLockTraceDistance`))) (`self.TargetLockTraceRadius`) (`self.TargetLockTraceObjectTypes`) false (`|MakeArray` (`self.GetOwner`)) (`self.TargetLockDebugDrawType`)))
  (return _outhits))