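; Actor component that lets its owner appear as a tracked marker on the player's radar widget in the Soulslike Framework.
; Add and remove events look up AC_RadarManager on the first player controller and pass this component to start or stop tracking, caching or clearing the returned marker widget.
; EndPlay removes the element automatically, while adding relies on an external call to the add event.
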(event `Event AddTrackedElement`
  (bind _returnvalue (`GameplayStatics.GetPlayerController` 0))
  (bind _returnvalue_2 (`Actor.GetComponentByClass` _returnvalue "/Game/SoulslikeFramework/Blueprints/Components/AC_RadarManager.AC_RadarManager_C"))
  ;[0.05098 0.05098 0.05098] Adds a new element to the radar widget and starts tracking it.
  (`/Engine/EditorBlueprintResources/StandardMacros.IsValid` _returnvalue
    (:`Is Valid`
      (`/Engine/EditorBlueprintResources/StandardMacros.IsValid` _returnvalue_2
        (:`Is Valid`
          (bind _trackedelementwidget (`/Game/SoulslikeFramework/Blueprints/Components/AC_RadarManager.StartTrackElement` _returnvalue_2 self))
          (`/Engine/EditorBlueprintResources/StandardMacros.IsValid` _trackedelementwidget
            (:`Is Valid`
              (set `self.MarkerWidget` _trackedelementwidget))))))))

(event `Event RemoveTrackedElement`
  (bind _returnvalue (`GameplayStatics.GetPlayerController` 0))
  (bind _returnvalue_2 (`Actor.GetComponentByClass` _returnvalue "/Game/SoulslikeFramework/Blueprints/Components/AC_RadarManager.AC_RadarManager_C"))
  ;[0.05098 0.05098 0.05098] Removes tracked element from the radar widget and stops tracking it.
  (`/Engine/EditorBlueprintResources/StandardMacros.IsValid` _returnvalue
    (:`Is Valid`
      (`/Engine/EditorBlueprintResources/StandardMacros.IsValid` _returnvalue_2
        (:`Is Valid`
          (`/Game/SoulslikeFramework/Blueprints/Components/AC_RadarManager.StopTrackElement` _returnvalue_2 self)
          (set `self.MarkerWidget` null))))))

(event `self.ReceiveEndPlay`
  (params (EndPlayReason :type "EEndPlayReason Enum" :default "Destroyed"))
  ;[0.05098 0.05098 0.05098] On EndPlay, remove all tracked elements.
  (`self.Event RemoveTrackedElement`))