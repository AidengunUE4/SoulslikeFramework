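; Actor component that manages an AI character's behavior state and blackboard in the Soulslike framework.
; On BeginPlay it starts the behavior tree, sets patrolling if a patrol path exists or else the default state, and pushes distance thresholds into blackboard keys.
; SetState tracks current and previous state and routes instanced-struct data to POI, target or patrol path.
; SetKeyValue writes any key type by probing the struct's type.
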(event `self.ReceiveBeginPlay`
  ;[0.05098 0.05098 0.05098] Initialize desired behavior tree
  (bind _behavior (`self.Behavior`)
    (:`then`
      (message `/Game/SoulslikeFramework/Blueprints/Interfaces/BPI_AIC.InitializeBehavior` (`AIBlueprintHelperLibrary.GetAIController` (`self.GetOwner`)) _behavior)
      ;[0.05098 0.05098 0.05098] If there's a valid patrol path actor, set state to patrolling and start immediately.
      (bind _patrolpath (`self.PatrolPath`)
        (:`then`
          (bind _returnvalue (`BlueprintInstancedStructLibrary.MakeInstancedStruct` (make `/Game/SoulslikeFramework/Structures/AI/FAiPatrolPathInfo` _patrolpath)))
          (`self.SetState` "NewEnumerator1" _returnvalue))
        (:`else`
          ;[0.05098 0.05098 0.05098] Otherwise use default state set.
          (`self.SetState` (`self.CurrentState`))))
      (`|ExecutionSequence`
        (:`then_0`
          ;[0.05098 0.05098 0.05098] Adjust ChaseDistance blackboard key
          (bind _returnvalue_2 (`BlueprintInstancedStructLibrary.MakeInstancedStruct` (make `/Game/SoulslikeFramework/Structures/_Misc/FFloat` (`self.MaxChaseDistanceThreshold`))))
          (`self.SetKeyValue` "ChaseDistance" _returnvalue_2))
        (:`then_1`
          ;[0.05098 0.05098 0.05098] Adjust AttackRadius blackboard key
          (bind _returnvalue_3 (`BlueprintInstancedStructLibrary.MakeInstancedStruct` (make `/Game/SoulslikeFramework/Structures/_Misc/FFloat` (`self.AttackDistanceThreshold`))))
          (`self.SetKeyValue` "AttackRadius" _returnvalue_3))
        (:`then_2`
          ;[0.05098 0.05098 0.05098] Adjust StrafeRadius blackboard key
          (bind _returnvalue_4 (`BlueprintInstancedStructLibrary.MakeInstancedStruct` (make `/Game/SoulslikeFramework/Structures/_Misc/FFloat` (`self.StrafeDistanceThreshold`))))
          (`self.SetKeyValue` "StrafeRadius" _returnvalue_4))
        (:`then_3`
          ;[0.05098 0.05098 0.05098] Adjust SpeedAdjustDistance blackboard key
          (bind _returnvalue_5 (`BlueprintInstancedStructLibrary.MakeInstancedStruct` (make `/Game/SoulslikeFramework/Structures/_Misc/FFloat` (`self.SpeedAdjustDistanceThreshold`))))
          (`self.SetKeyValue` "SpeedAdjustDistance" _returnvalue_5))))
    (:`else`)))

(fn `GetBlackboard`
  (returns (ReturnValue :type "BlackboardComponent Object Reference"))
  (bind _returnvalue (`AIBlueprintHelperLibrary.GetBlackboard` (`AIBlueprintHelperLibrary.GetAIController` (`self.GetOwner`))))
  ;[0.05098 0.05098 0.05098] Retrieves Blackboard asset from Owner's AIController.
  (`/Engine/EditorBlueprintResources/StandardMacros.IsValid` _returnvalue
    (:`Is Valid`
      (return _returnvalue))
    (:`Is Not Valid`
      (return null))))

(fn `GetState`
  (params (Handle :type "/Game/SoulslikeFramework/Enums/E_AI_StateHandle Enum" :default "NewEnumerator0"))
  (returns (State :type "/Game/SoulslikeFramework/Enums/E_AI_States Enum"))
  ;[0.05098 0.05098 0.05098] Simple state getter
  (return (select `/Game/SoulslikeFramework/Enums/E_AI_StateHandle` Handle :`NewEnumerator0` (`self.CurrentState`) :`NewEnumerator4` (`self.PreviousState`))))

(fn `GetTarget`
  (returns (Target :type "Actor Object Reference"))
  (locals (LOCAL_CurrentState :type "/Game/SoulslikeFramework/Enums/E_AI_States Enum" :default "NewEnumerator0"))
  ;[0.05098 0.05098 0.05098] Simple getter for current target
  (return (`self.CurrentTarget`)))

(fn `SetKeyValue`
  (params (KeyName :type Name) (Data :type "InstancedStruct Structure"))
  ;[0.05098 0.05098 0.05098] Method to set any blackboard key through the usage of instanced structs
  (bind _value (`BlueprintInstancedStructLibrary.GetInstancedStructValue` (`local.Data`))
    (:`Valid`
      (`BlackboardComponent.SetValueAsBool` (`self.GetBlackboard`) (`local.KeyName`) (`.Bool_1_34B002874AE3A0F647800E9B1FC501EA` (break `/Game/SoulslikeFramework/Structures/_Misc/FBool` _value))))
    (:`NotValid`
      (bind _value_2 (`BlueprintInstancedStructLibrary.GetInstancedStructValue` (`local.Data`))
        (:`Valid`
          (`BlackboardComponent.SetValueAsClass` (`self.GetBlackboard`) (`local.KeyName`) (`.Class_4_AA7DF68F4132A8DB674BA4ACB97810E4` (break `/Game/SoulslikeFramework/Structures/_Misc/FClass` _value_2))))
        (:`NotValid`
          (bind _value_3 (`BlueprintInstancedStructLibrary.GetInstancedStructValue` (`local.Data`))
            (:`Valid`
              (`BlackboardComponent.SetValueAsEnum` (`self.GetBlackboard`) (`local.KeyName`) (`.Enum_7_1A78F71247A43162364DD596F5E8DC2E` (break `/Game/SoulslikeFramework/Structures/_Misc/FEnumByte` _value_3))))
            (:`NotValid`
              (bind _value_4 (`BlueprintInstancedStructLibrary.GetInstancedStructValue` (`local.Data`))
                (:`Valid`
                  (`BlackboardComponent.SetValueAsFloat` (`self.GetBlackboard`) (`local.KeyName`) (`.Float_10_1635518D4B5EA126D75B9481FB7F017E` (break `/Game/SoulslikeFramework/Structures/_Misc/FFloat` _value_4))))
                (:`NotValid`
                  (bind _value_5 (`BlueprintInstancedStructLibrary.GetInstancedStructValue` (`local.Data`))
                    (:`Valid`
                      (`BlackboardComponent.SetValueAsInt` (`self.GetBlackboard`) (`local.KeyName`) (`.Int_31_1635518D4B5EA126D75B9481FB7F017E` (break `/Game/SoulslikeFramework/Structures/_Misc/FInt` _value_5))))
                    (:`NotValid`
                      (bind _value_6 (`BlueprintInstancedStructLibrary.GetInstancedStructValue` (`local.Data`))
                        (:`Valid`
                          (`BlackboardComponent.SetValueAsName` (`self.GetBlackboard`) (`local.KeyName`) (`.Name_16_8D91767A45C55C0A29AF94AF39968A8A` (break `/Game/SoulslikeFramework/Structures/_Misc/FName` _value_6))))
                        (:`NotValid`
                          (bind _value_7 (`BlueprintInstancedStructLibrary.GetInstancedStructValue` (`local.Data`))
                            (:`Valid`
                              (`BlackboardComponent.SetValueAsObject` (`self.GetBlackboard`) (`local.KeyName`) (`.Object_31_D9BBE3904823C7235805F08EE8982FA8` (break `/Game/SoulslikeFramework/Structures/_Misc/FObject` _value_7))))
                            (:`NotValid`
                              (bind _value_8 (`BlueprintInstancedStructLibrary.GetInstancedStructValue` (`local.Data`))
                                (:`Valid`
                                  (`BlackboardComponent.SetValueAsRotator` (`self.GetBlackboard`) (`local.KeyName`) (`.Rotator_29_710E3F0F4CFA8BA74D31ECA092A376E0` (break `/Game/SoulslikeFramework/Structures/_Misc/FRotator` _value_8))))
                                (:`NotValid`
                                  (bind _value_9 (`BlueprintInstancedStructLibrary.GetInstancedStructValue` (`local.Data`))
                                    (:`Valid`
                                      (`BlackboardComponent.SetValueAsString` (`self.GetBlackboard`) (`local.KeyName`) (`.String_28_C01889024086FC25EBB6FD91069C3A9D` (break `/Game/SoulslikeFramework/Structures/_Misc/FString` _value_9))))
                                    (:`NotValid`
                                      (bind _value_10 (`BlueprintInstancedStructLibrary.GetInstancedStructValue` (`local.Data`))
                                        (:`Valid`
                                          (`BlackboardComponent.SetValueAsVector` (`self.GetBlackboard`) (`local.KeyName`) (`.Vector_27_D9BBE3904823C7235805F08EE8982FA8` (break `/Game/SoulslikeFramework/Structures/_Misc/FVector` _value_10))))))))))))))))))))))))

(fn `SetPatrolPath`
  (params (PatrolPath :type "/Game/SoulslikeFramework/Blueprints/_AI/Misc/B_PatrolPath Object Reference"))
  (locals (LOCAL_CurrentState :type "/Game/SoulslikeFramework/Enums/E_AI_States Enum" :default "NewEnumerator0"))
  ;[0.05098 0.05098 0.05098] Sets patrol path actor property
  (set `self.PatrolPath` PatrolPath))

(fn `SetState`
  (params (NewState :type "/Game/SoulslikeFramework/Enums/E_AI_States Enum" :default "NewEnumerator0") (Data :type "InstancedStruct Structure"))
  ;[0.05098 0.05098 0.05098] Method to set AI state. Will set current state to previous state and adjust current state. Afterwards, will do 3 generic checks for incoming Data. Feel free to extend this to your needs.
  (`/Engine/EditorBlueprintResources/StandardMacros.IsValid` (`self.GetBlackboard`)
    (:`Is Valid`
      (`|ExecutionSequence`
        (:`then_0`
          (set `self.PreviousState` (`self.CurrentState`))
          (bind _output_get (set `self.CurrentState` (`local.NewState`)))
          (`BlackboardComponent.SetValueAsEnum` (`self.GetBlackboard`) "State" _output_get))
        (:`then_1`
          (`BlueprintInstancedStructLibrary.IsInstancedStructValid` (`local.Data`)
            (:`Valid`
              (bind _value (`BlueprintInstancedStructLibrary.GetInstancedStructValue` (`local.Data`))
                (:`Valid`
                  (bind _returnvalue (`BlueprintInstancedStructLibrary.MakeInstancedStruct` (make `/Game/SoulslikeFramework/Structures/_Misc/FVector` (`.SenseLocation_2_552EA7DE4E62FC30D471519DF580AA24` (break `/Game/SoulslikeFramework/Structures/AI/FAiSenseLocationInfo` _value)))))
                  (`self.SetKeyValue` "POI" _returnvalue))
                (:`NotValid`
                  (bind _value_2 (`BlueprintInstancedStructLibrary.GetInstancedStructValue` (`local.Data`))
                    (:`Valid`
                      (`self.SetTarget` (`.SensedTarget_4_552EA7DE4E62FC30D471519DF580AA24` (break `/Game/SoulslikeFramework/Structures/AI/FAiSenseTargetInfo` _value_2))))
                    (:`NotValid`
                      (bind _value_3 (`BlueprintInstancedStructLibrary.GetInstancedStructValue` (`local.Data`))
                        (:`Valid`
                          (`self.SetPatrolPath` (`.PatrolPath_6_552EA7DE4E62FC30D471519DF580AA24` (break `/Game/SoulslikeFramework/Structures/AI/FAiPatrolPathInfo` _value_3))))))))))))))))

(fn `SetTarget`
  (params (Target :type "Actor Object Reference"))
  (locals (LOCAL_CurrentState :type "/Game/SoulslikeFramework/Enums/E_AI_States Enum" :default "NewEnumerator0"))
  ;[0.05098 0.05098 0.05098] Sets current target property and also key value
  (bind _output_get (set `self.CurrentTarget` Target))
  (bind _returnvalue (`BlueprintInstancedStructLibrary.MakeInstancedStruct` (make `/Game/SoulslikeFramework/Structures/_Misc/FObject` _output_get)))
  (`self.SetKeyValue` "Target" _returnvalue))