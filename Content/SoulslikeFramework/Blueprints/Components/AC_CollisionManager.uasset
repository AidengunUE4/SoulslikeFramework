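; Weapon collision component that detects melee hits by sweeping between two sockets on the owner's static or skeletal mesh.
; ToggleTrace clears the hit list and enables Tick, which runs substepped sphere traces lerped from last frame's socket positions, so fast swings leave no gaps.
; ProcessTrace broadcasts OnActorTraced once per actor per activation with the damage multiplier.
; Adjustable multipliers scale damage and trace radius, and debug drawing is optional.
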(event `self.ReceiveBeginPlay`
  (bind _returnvalue (`self.GetOwner`))
  (bind _returnvalue_2 (`Actor.GetComponentByClass` _returnvalue "/Script/Engine.StaticMeshComponent"))
  ;[0.05098 0.05098 0.05098] Starts a timer on BeginPlay and pauses it. This timer is controlled with animation notifies.
  (set `self.TargetMesh` (select `bool` (`KismetSystemLibrary.IsValid` _returnvalue_2) :`false` (`Actor.GetComponentByClass` _returnvalue "/Script/Engine.SkeletalMeshComponent") :`true` _returnvalue_2 :!type "SceneComponent Object Reference")))

(event `Event InitializeTracePoints`
  (bind (_trace_start_location _trace_end_location) (`self.GetTraceLocations`))
  ;[0.05098 0.05098 0.05098] Starts a timer on BeginPlay and pauses it. This timer is controlled with animation notifies.
  (set `self.LastStartPosition` _trace_start_location)
  (set `self.LastEndPosition` _trace_end_location))

(event `self.ReceiveTick`
  (params (DeltaSeconds :type "Float (single-precision)"))
  ;[0.05098 0.05098 0.05098] Substepped weapon trace using time slicing
  (`self.SubsteppedTrace` (* (`self.TraceRadius`) (`self.TraceSizeMultiplier`))))

(event `Event ToggleTrace`
  (params (`Enabled?` :type Boolean))
  ;[0.05098 0.05098 0.05098] Event to toggle tracing on/off
  (if `Enabled?`
    (`KismetArrayLibrary.Array_Clear` (`self.TracedActors`))
    (`self.SetComponentTickEnabled` true)
    (`self.Event InitializeTracePoints`)
    (else
      (`self.SetComponentTickEnabled` false))))

(fn `GetMultipliers`
  (returns (DamageMultiplier :type "Float (double-precision)") (TraceSizeMultiplier :type "Float (double-precision)"))
  ;[0.05098 0.05098 0.05098] Simply retrieves current damage multiplier
  (return (`self.DamageMultiplier`) (`self.TraceSizeMultiplier`)))

(fn `GetTraceLocations`
  (returns (`Trace Start Location` :type "Vector Structure") (`Trace End Location` :type "Vector Structure"))
  (locals (LOCAL_StartLoc :type "Vector Structure" :default (0.0 0.0 0.0)) (LOCAL_EndLoc :type "Vector Structure" :default (0.0 0.0 0.0)))
  (bind _targetmesh (`self.TargetMesh`))
  ;[0.05098 0.05098 0.05098] Gets trace locations from weapon mesh's sockets.
  (set `local.LOCAL_StartLoc` (`SceneComponent.GetSocketLocation` _targetmesh (`self.TraceSocketStart`)))
  (set `local.LOCAL_EndLoc` (`SceneComponent.GetSocketLocation` _targetmesh (`self.TraceSocketEnd`)))
  (return (`local.LOCAL_StartLoc`) (`local.LOCAL_EndLoc`)))

(fn `ProcessTrace`
  (params (Hits :type "Array of HitResult Structure"))
  ;[0.05098 0.05098 0.05098] Checks if hit actor has already been traced. This ensures that a weapon only damages an actor once.
  (for _array_element Hits
    (bind (_bblockinghit _binitialoverlap _time _distance _location _impactpoint _normal _impactnormal _physmat _hitactor) (`GameplayStatics.BreakHitResult` _array_element))
    (if (not (`KismetArrayLibrary.Array_Contains` (`self.TracedActors`) _hitactor))
      (`KismetArrayLibrary.Array_Add` (`self.TracedActors`) _hitactor)
      (`self.OnActorTraced` _hitactor _array_element (`self.DamageMultiplier`)))))

(fn `SetMultipliers`
  (params (DamageMultiplier :type "Float (double-precision)" :default 1.0) (TraceSizeMultiplier :type "Float (double-precision)" :default 1.0))
  ;[0.05098 0.05098 0.05098] Simply sets a damage and a trace size multiplier
  (set `self.DamageMultiplier` DamageMultiplier)
  (set `self.TraceSizeMultiplier` TraceSizeMultiplier))

(fn `SubsteppedTrace`
  (params (StepSize :type "Float (double-precision)"))
  (locals (LOCAL_CurrentStartPosition :type "Vector Structure" :default (0.0 0.0 0.0)) (LOCAL_CurrentEndPosition :type "Vector Structure" :default (0.0 0.0 0.0)) (LOCAL_Distance :type "Float (double-precision)") (LOCAL_Substeps :type Integer) (LOCAL_Alpha :type "Float (double-precision)") (LOCAL_NewStartPosition :type "Vector Structure") (LOCAL_NewEndPosition :type "Vector Structure"))
  (bind (_trace_start_location _trace_end_location) (`self.GetTraceLocations`))
  (bind _returnvalue (`self.GetOwner`))
  ;[0.05098 0.05098 0.05098] Cache current socket positions of the weapon as Start & End
  (set `local.LOCAL_CurrentStartPosition` _trace_start_location)
  (set `local.LOCAL_CurrentEndPosition` _trace_end_location)
  ;[0.05098 0.05098 0.05098] Calculate distance & required substeps for the tracing.
  (bind _output_get (set `local.LOCAL_Distance` (`KismetMathLibrary.Vector_Distance` (`self.LastStartPosition`) (`local.LOCAL_CurrentStartPosition`))))
  (bind _output_get_2 (set `local.LOCAL_Substeps` (`KismetMathLibrary.Max` (`KismetMathLibrary.FCeil` (/ _output_get (`local.StepSize`))) 1)))
  ;[0.05098 0.05098 0.05098] Foreach substep, lerp from last Start & End positions to current Start & End positions, doing a multi sphere trace along the way.
  (for _index (range (+ _output_get_2 1))
    (set `local.LOCAL_Alpha` (/ (`KismetMathLibrary.Conv_IntToDouble` _index) (`local.LOCAL_Substeps`)))
    (set `local.LOCAL_NewStartPosition` (`KismetMathLibrary.VLerp` (`self.LastStartPosition`) (`local.LOCAL_CurrentStartPosition`) (`local.LOCAL_Alpha`)))
    (set `local.LOCAL_NewEndPosition` (`KismetMathLibrary.VLerp` (`self.LastEndPosition`) (`local.LOCAL_CurrentEndPosition`) (`local.LOCAL_Alpha`)))
    (bind (_outhits _returnvalue_2) (`KismetSystemLibrary.SphereTraceMultiForObjects` (`local.LOCAL_NewStartPosition`) (`local.LOCAL_NewEndPosition`) (* (`self.TraceRadius`) (`self.TraceSizeMultiplier`)) (`self.TraceTypes`) false (`|MakeArray` _returnvalue (`Actor.Instigator` _returnvalue) :!type "Actor Object Reference") (`self.TraceDebugMode`)))
    (if _returnvalue_2
      (`self.ProcessTrace` _outhits)))
  ;[0.05098 0.05098 0.05098] Reset last start & end positions.
  (if (`|EnumInequality` (`self.TraceDebugMode`))
    (`KismetSystemLibrary.DrawDebugLine` (`self.LastStartPosition`) (`local.LOCAL_CurrentStartPosition`) (struct :`R` 1.0 :`G` 0.664457 :`A` 1.0) 1.0 2.0))
  (set `self.LastStartPosition` (`local.LOCAL_CurrentStartPosition`))
  (set `self.LastEndPosition` (`local.LOCAL_CurrentEndPosition`)))