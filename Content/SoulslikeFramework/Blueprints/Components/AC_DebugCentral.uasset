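; Debug component that gives a Soulslike character an on-screen debug HUD with a toggleable control panel, active only when debugging is enabled.
; After a short startup delay, it gathers the framework's manager components from the owner and its controller into a tag-keyed map and passes it to the HUD widget.
; Tick polls the toggle key directly, switching panel visibility, mouse cursor and input mode, debounced with a DoOnce and delay.
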(event `self.ReceiveBeginPlay`
  ;[0.05098 0.05098 0.05098] If debugging is enabled, enable tick. Otherwise, disable tick.
  (if (`self.EnableDebugging`)
    (`KismetSystemLibrary.K2_SetTimerDelegate` (delegate `LateInitialize`) 2.0)
    (`self.SetComponentTickEnabled` true)
    (else
      (`self.SetComponentTickEnabled` false))))

(event `LateInitialize`
  (bind _returnvalue (`self.GetOwner`))
  (bind _returnvalue_2 (`Pawn.GetController` (`Actor.Instigator` (`self.GetOwner`))))
  ;[0.05098 0.05098 0.05098] Initialize a bit late to allow all components and widgets to initialize.
  (if (`GameplayStatics.ObjectIsA` (`self.GetOwner`) "/Game/SoulslikeFramework/Blueprints/_Characters/B_Soulslike_Character.B_Soulslike_Character_C")
    (`BlueprintMapLibrary.Map_Clear` (`self.Components`))
    (bind _output_get (set `self.StatusEffectComponent` (`Actor.GetComponentByClass` _returnvalue "/Game/SoulslikeFramework/Blueprints/Components/AC_StatusEffectManager.AC_StatusEffectManager_C")))
    (`BlueprintMapLibrary.Map_Add` (`self.Components`) (struct :`TagName` "SoulslikeFramework.Backend.Components.StatusEffect") _output_get)
    (bind _output_get_2 (set `self.StatComponent` (`Actor.GetComponentByClass` _returnvalue "/Game/SoulslikeFramework/Blueprints/Components/AC_StatManager.AC_StatManager_C")))
    (`BlueprintMapLibrary.Map_Add` (`self.Components`) (struct :`TagName` "SoulslikeFramework.Backend.Components.Stat") _output_get_2)
    (bind _output_get_3 (set `self.CombatComponent` (`Actor.GetComponentByClass` _returnvalue "/Game/SoulslikeFramework/Blueprints/Components/AC_CombatManager.AC_CombatManager_C")))
    (`BlueprintMapLibrary.Map_Add` (`self.Components`) (struct :`TagName` "SoulslikeFramework.Backend.Components.Combat") _output_get_3)
    (bind _output_get_4 (set `self.ActionComponent` (`Actor.GetComponentByClass` _returnvalue "/Game/SoulslikeFramework/Blueprints/Components/AC_ActionManager.AC_ActionManager_C")))
    (`BlueprintMapLibrary.Map_Add` (`self.Components`) (struct :`TagName` "SoulslikeFramework.Backend.Components.Action") _output_get_4)
    (bind _output_get_5 (set `self.InteractionComponent` (`Actor.GetComponentByClass` _returnvalue "/Game/SoulslikeFramework/Blueprints/Components/AC_InteractionManager.AC_InteractionManager_C")))
    (`BlueprintMapLibrary.Map_Add` (`self.Components`) (struct :`TagName` "SoulslikeFramework.Backend.Components.Interaction") _output_get_5)
    (bind _output_get_6 (set `self.BuffComponent` (`Actor.GetComponentByClass` _returnvalue "/Game/SoulslikeFramework/Blueprints/Components/AC_BuffManager.AC_BuffManager_C")))
    (`BlueprintMapLibrary.Map_Add` (`self.Components`) (struct :`TagName` "SoulslikeFramework.Backend.Components.Buff") _output_get_6)
    (bind _output_get_7 (set `self.InputComponent` (`Actor.GetComponentByClass` _returnvalue "/Game/SoulslikeFramework/Blueprints/Components/AC_InputBuffer.AC_InputBuffer_C")))
    (`BlueprintMapLibrary.Map_Add` (`self.Components`) (struct :`TagName` "SoulslikeFramework.Backend.Components.Input") _output_get_7)
    (bind _output_get_8 (set `self.EquipmentComponent` (`Actor.GetComponentByClass` _returnvalue_2 "/Game/SoulslikeFramework/Blueprints/Components/AC_EquipmentManager.AC_EquipmentManager_C")))
    (`BlueprintMapLibrary.Map_Add` (`self.Components`) (struct :`TagName` "SoulslikeFramework.Backend.Components.Equipment") _output_get_8)
    (bind _output_get_9 (set `self.InventoryComponent` (`Actor.GetComponentByClass` _returnvalue_2 "/Game/SoulslikeFramework/Blueprints/Components/AC_InventoryManager.AC_InventoryManager_C")))
    (`BlueprintMapLibrary.Map_Add` (`self.Components`) (struct :`TagName` "SoulslikeFramework.Backend.Components.Inventory") _output_get_9)
    (bind _output_get_10 (set `self.RadarComponent` (`Actor.GetComponentByClass` _returnvalue_2 "/Game/SoulslikeFramework/Blueprints/Components/AC_RadarManager.AC_RadarManager_C")))
    (`BlueprintMapLibrary.Map_Add` (`self.Components`) (struct :`TagName` "SoulslikeFramework.Backend.Components.Radar") _output_get_10)
    (bind _output_get_11 (set `self.ProgressComponent` (`Actor.GetComponentByClass` _returnvalue_2 "/Game/SoulslikeFramework/Blueprints/Components/AC_ProgressManager.AC_ProgressManager_C")))
    (`BlueprintMapLibrary.Map_Add` (`self.Components`) (struct :`TagName` "SoulslikeFramework.Backend.Components.Progress") _output_get_11)
    (bind _output_get_12 (set `self.SaveLoadComponent` (`Actor.GetComponentByClass` _returnvalue_2 "/Game/SoulslikeFramework/Blueprints/Components/AC_SaveLoadManager.AC_SaveLoadManager_C")))
    (`BlueprintMapLibrary.Map_Add` (`self.Components`) (struct :`TagName` "SoulslikeFramework.Backend.Components.SaveLoad") _output_get_12)
    (bind _returnvalue_3 (`|CreateWidget` "/Game/SoulslikeFramework/Widgets/_Debug/W_Debug_HUD.W_Debug_HUD_C" null (`self.Components`)))
    (bind _output_get_13 (set `self.HUD_Debug` _returnvalue_3))
    (`/Game/SoulslikeFramework/Widgets/_Debug/W_Debug_HUD.Event InitializeText` _output_get_13 (`self.ToggleKey`))
    (`UserWidget.AddToViewport` _output_get_13 0)))

(event `self.ReceiveTick`
  (params (DeltaSeconds :type "Float (single-precision)"))
  (bind _returnvalue (`GameplayStatics.GetPlayerController` 0))
  (bind _returnvalue_2 (`GameplayStatics.GetPlayerController` 0))
  ;[0.05098 0.05098 0.05098] Handle input manually thru tick event
  (`|ExecutionSequence`
    (:`then_1`
      (`self.HUD_Debug`
        (:`then`
          (if (> (`PlayerController.GetInputKeyTimeDown` (`GameplayStatics.GetPlayerController` 0) (`self.ToggleKey`)) 0.05)
            (`/Engine/EditorBlueprintResources/StandardMacros.DoOnce` false :!label _label
              (:`Completed`
                (if (`Widget.IsVisible` (`/Game/SoulslikeFramework/Widgets/_Debug/W_Debug_HUD.ControlPanel` (`self.HUD_Debug`)))
                  (set `PlayerController.bShowMouseCursor` false _returnvalue_2)
                  (`WidgetBlueprintLibrary.SetInputMode_GameOnly` _returnvalue_2 true)
                  (else
                    (set `PlayerController.bShowMouseCursor` true _returnvalue)
                    (`WidgetBlueprintLibrary.SetInputMode_GameAndUIEx` _returnvalue (`/Game/SoulslikeFramework/Widgets/_Debug/W_Debug_HUD.ControlPanel` (`self.HUD_Debug`)) "DoNotLock" true true)))
                (`Widget.SetVisibility` (`/Game/SoulslikeFramework/Widgets/_Debug/W_Debug_HUD.ControlPanel` (`self.HUD_Debug`)) (select `bool` (`Widget.IsVisible` (`/Game/SoulslikeFramework/Widgets/_Debug/W_Debug_HUD.ControlPanel` (`self.HUD_Debug`))) :`false` "Visible" :`true` "Collapsed" :!type "ESlateVisibility Enum"))
                (`KismetSystemLibrary.Delay` 0.2)
                (goto _label :!via `Reset`)))))
        (:`else`)))))