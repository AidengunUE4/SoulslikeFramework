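; Actor component that manages Soulslike status effects on its owner, tracking active effects in a map keyed by tag.
; Start, stop and one-shot buildup calls update the existing effect, or async-load and construct a B_StatusEffect object from its data when none is tracked.
; Each effect reports back when triggered or finished, and the component broadcasts added, removed and triggered dispatchers, the latter feeding W_StatusEffectNotification.
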(event `Event TryAddStatusEffect`
  (params (`Effect Class` :type "/Game/SoulslikeFramework/Data/StatusEffects/StatusEffectData/PDA_StatusEffect Object Reference") (Rank :type Integer) (`StartBuildup?` :type Boolean :default true) (StartAmount :type "Float (double-precision)"))
  ;[0.05098 0.05098 0.05098] If Status Effect is not active, construct relevant Status Effect object and initialize it. Also start tracking it.
  (`KismetSystemLibrary.Delay` 0.1)
  (`/Engine/EditorBlueprintResources/StandardMacros.IsValid` `Effect Class`
    (:`Is Valid`
      (if (not (`BlueprintMapLibrary.Map_Contains` (`self.ActiveStatusEffects`) (`/Game/SoulslikeFramework/Data/StatusEffects/StatusEffectData/PDA_StatusEffect.Tag` `Effect Class`)))
        (bind _effect (`/Game/SoulslikeFramework/Data/StatusEffects/StatusEffectData/PDA_StatusEffect.Effect` `Effect Class`)
          (:`then`
            (bind _class (`|LoadAssetClass` _effect)
              (:`Completed`
                (bind _asstatus_effect_object (castclass `/Game/SoulslikeFramework/Data/StatusEffects/StatusEffectClasses/B_StatusEffect` _class))
                (bind _returnvalue (`|GenericCreateObject` _asstatus_effect_object (`self.GetOwner`) `Effect Class`))
                (`BlueprintMapLibrary.Map_Add` (`self.ActiveStatusEffects`) (`/Game/SoulslikeFramework/Data/StatusEffects/StatusEffectData/PDA_StatusEffect.Tag` `Effect Class`) _returnvalue)
                (`self.OnStatusEffectAdded` _returnvalue)
                (add `/Game/SoulslikeFramework/Data/StatusEffects/StatusEffectClasses/B_StatusEffect.OnStatusEffectTriggered` _returnvalue (`|CreateDelegate` :!event `Event OnStatusEffectTriggered`))
                (add `/Game/SoulslikeFramework/Data/StatusEffects/StatusEffectClasses/B_StatusEffect.OnStatusEffectFinished` _returnvalue (`|CreateDelegate` :!event `Event OnStatusEffectFinished`))
                (`/Game/SoulslikeFramework/Data/StatusEffects/StatusEffectClasses/B_StatusEffect.Event Initialize` _returnvalue Rank)
                (if `StartBuildup?`
                  (`/Game/SoulslikeFramework/Data/StatusEffects/StatusEffectClasses/B_StatusEffect.Event StartBuildup` _returnvalue)
                  (else
                    (`/Game/SoulslikeFramework/Data/StatusEffects/StatusEffectClasses/B_StatusEffect.Event AdjustBuildupOneshot` _returnvalue StartAmount))))))
          (:`else`))))))

(event `Event OnStatusEffectFinished`
  (params (StatusEffectTag :type "GameplayTag Structure"))
  (bind (_value _returnvalue) (`BlueprintMapLibrary.Map_Find` (`self.ActiveStatusEffects`) StatusEffectTag))
  ;[0.05098 0.05098 0.05098] When finished, remove from tracking map
  (if _returnvalue
    (`self.OnStatusEffectRemoved` (`/Game/SoulslikeFramework/Data/StatusEffects/StatusEffectClasses/B_StatusEffect.Data` _value))
    (`BlueprintMapLibrary.Map_Remove` (`self.ActiveStatusEffects`) StatusEffectTag)))

(event `Event OnStatusEffectTriggered`
  (params (TriggeredText :type Text))
  ;[0.05098 0.05098 0.05098] When a status effect is triggered, call this dispatcher which is being listened by W_StatusEffectNotification
  (`self.OnStatusEffectTriggered` TriggeredText))

(fn `AddOneShotBuildup`
  (params (StatusEffect :type "/Game/SoulslikeFramework/Data/StatusEffects/StatusEffectData/PDA_StatusEffect Object Reference") (EffectRank :type Integer) (Delta :type "Float (double-precision)"))
  (bind _delta (`local.Delta`))
  (bind _effectrank (`local.EffectRank`))
  (bind (_value _returnvalue) (`BlueprintMapLibrary.Map_Find` (`self.ActiveStatusEffects`) (`/Game/SoulslikeFramework/Data/StatusEffects/StatusEffectData/PDA_StatusEffect.Tag` StatusEffect)))
  ;[0.05098 0.05098 0.05098] Adds delta buildup to target status effect with rank
  (`/Engine/EditorBlueprintResources/StandardMacros.IsValid` StatusEffect
    (:`Is Valid`
      (if _returnvalue
        (`/Game/SoulslikeFramework/Data/StatusEffects/StatusEffectClasses/B_StatusEffect.Event RefreshRank` _value _effectrank)
        (`/Game/SoulslikeFramework/Data/StatusEffects/StatusEffectClasses/B_StatusEffect.Event AdjustBuildupOneshot` _value _delta)
        (else
          (`self.Event TryAddStatusEffect` (`local.StatusEffect`) _effectrank false _delta))))))

(fn `IsStatusEffectActive`
  (params (StatusEffectTag :type "GameplayTag Structure"))
  (returns (ReturnValue :type Boolean))
  (bind (_value _returnvalue) (`BlueprintMapLibrary.Map_Find` (`self.ActiveStatusEffects`) StatusEffectTag))
  ;[0.05098 0.05098 0.05098] Checks if a status effect is active (triggered) by its tag
  (if _returnvalue
    (return (`/Game/SoulslikeFramework/Data/StatusEffects/StatusEffectClasses/B_StatusEffect.IsTriggered?` _value))))

(fn `StartBuildup`
  (params (StatusEffect :type "/Game/SoulslikeFramework/Data/StatusEffects/StatusEffectData/PDA_StatusEffect Object Reference") (Rank :type Integer))
  (bind _rank (`local.Rank`))
  (bind (_value _returnvalue) (`BlueprintMapLibrary.Map_Find` (`self.ActiveStatusEffects`) (`/Game/SoulslikeFramework/Data/StatusEffects/StatusEffectData/PDA_StatusEffect.Tag` StatusEffect)))
  ;[0.05098 0.05098 0.05098] Starts buildup of target status effect with rank.
  (`/Engine/EditorBlueprintResources/StandardMacros.IsValid` StatusEffect
    (:`Is Valid`
      (if _returnvalue
        (`/Game/SoulslikeFramework/Data/StatusEffects/StatusEffectClasses/B_StatusEffect.Event RefreshRank` _value _rank)
        (`/Game/SoulslikeFramework/Data/StatusEffects/StatusEffectClasses/B_StatusEffect.Event StartBuildup` _value)
        (else
          (`self.Event TryAddStatusEffect` (`local.StatusEffect`) _rank))))))

(fn `StopBuildup`
  (params (StatusEffect :type "/Game/SoulslikeFramework/Data/StatusEffects/StatusEffectData/PDA_StatusEffect Object Reference") (`ApplyDecayDelay?` :type Boolean :default true))
  (bind (_value _returnvalue) (`BlueprintMapLibrary.Map_Find` (`self.ActiveStatusEffects`) (`/Game/SoulslikeFramework/Data/StatusEffects/StatusEffectData/PDA_StatusEffect.Tag` StatusEffect)))
  ;[0.05098 0.05098 0.05098] Stops buildup of Status Effect
  (`/Engine/EditorBlueprintResources/StandardMacros.IsValid` StatusEffect
    (:`Is Valid`
      (if _returnvalue
        (`/Game/SoulslikeFramework/Data/StatusEffects/StatusEffectClasses/B_StatusEffect.Event StopBuildup` _value `ApplyDecayDelay?`)))))