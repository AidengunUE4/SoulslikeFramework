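; Input buffer component for Soulslike characters that holds an action requested mid-action, such as a light attack during a dodge, until it can play.
; QueueAction consumes immediately when the buffer is closed; while open, QueueNext rechecks each tick until it closes, skipping tags in IgnoreNextOfActions.
; Consuming broadcasts the action tag through OnInputBufferConsumed for B_SoulslikeCharacter, then clears it.
; ExecuteActionImmediately bypasses the wait, and ToggleBuffer sets the open state.
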(event `Event QueueNext`
  (params (ActionTag :type "GameplayTag Structure"))
  ;[0.05098 0.05098 0.05098] Queues next action. For e.g, if player is dodging and at the same time tries to do a Light Attack, it will be queued and played when possible.
  (if (not (`BlueprintGameplayTagLibrary.HasTag` (`self.IgnoreNextOfActions`) ActionTag))
    (if (`self.BufferOpen?`) :!label _label
      (`KismetSystemLibrary.DelayUntilNextTick`)
      (goto _label)
      (else
        (set `self.IncomingActionTag` ActionTag)
        (`self.ConsumeInputBuffer`)))))

(fn `ConsumeInputBuffer`
  ;[0.05098 0.05098 0.05098] On consumed, resets Incoming Action tag. The dispatcher is utilised inside B_SoulslikeCharacter.
  (`self.OnInputBufferConsumed` (`self.IncomingActionTag`))
  (set `self.IncomingActionTag` (struct)))

(fn `ExecuteActionImmediately`
  (params (Action :type "GameplayTag Structure"))
  ;[0.05098 0.05098 0.05098] Immediately consumes buffer.
  (set `self.IncomingActionTag` Action)
  (`self.ConsumeInputBuffer`))

(fn `QueueAction`
  (params (QueuedActionTag :type "GameplayTag Structure"))
  ;[0.05098 0.05098 0.05098] Queues action
  (bind _output_get (set `self.IncomingActionTag` QueuedActionTag))
  ;;[0.05098 0.05098 0.05098] If buffer is closed, consume immediately.
  (if (`self.BufferOpen?`)
    (`self.Event QueueNext` _output_get)
    (else
      (`self.ConsumeInputBuffer`))))

(fn `ToggleBuffer`
  (params (`BufferOpen?` :type Boolean))
  ;[0.05098 0.05098 0.05098] Toggle buffer on/off
  (set `self.BufferOpen?` `BufferOpen?`))