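; Player controller component that drives a compass-style radar strip, showing the player icon, cardinal directions and markers for tracked actors with AC_RadarElement.
; Initialize populates the radar widget and creates a looping, initially paused refresh timer that ToggleUpdateState controls.
; Refreshes convert the signed yaw delta between camera and each target into horizontal translation, scaled by camera FOV and clamp length.
; Entries outside that range are collapsed.
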(event `Event Initialize`
  (params (RadarWidget :type "/Game/SoulslikeFramework/Widgets/Radar/W_Radar Object Reference") (Pawn :type "Pawn Object Reference"))
  ;[0.05098 0.05098 0.05098] Initialize Radar widget and add desired cardinals. Called from PC_SoulslikeFramework (player controller).
  (set `self.RadarWidget` RadarWidget)
  (bind _output_get (set `self.Pawn` Pawn))
  (set `self.PlayerCamera` (`Actor.GetComponentByClass` _output_get "/Script/Engine.CameraComponent"))
  (`self.SetupPlayerIcon`)
  (`self.SetupCardinals`)
  (`self.Event SetupUpdateTimer`))

(event `Event SetupUpdateTimer`
  ;[0.05098 0.05098 0.05098] Update timer - will get enabled/disabled (paused/unpaused) depending on camera movement
  (bind _returnvalue (`KismetSystemLibrary.K2_SetTimerDelegate` (`|CreateDelegate` :!event `Event UpdateVisuals`) (`self.RefreshInterval`) true))
  (bind _output_get (set `self.Timer` _returnvalue))
  (`KismetSystemLibrary.K2_PauseTimerHandle` _output_get))

(event `Event UpdateVisuals`
  ;[0.05098 0.05098 0.05098] Update timer - will get enabled/disabled (paused/unpaused) depending on camera movement
  (`self.RefreshCardinals`)
  (`self.RefreshTrackedElements`))

(fn `ConvertToCircleDegrees`
  (params (In :type "Float (double-precision)"))
  (returns (ReturnValue :type "Float (double-precision)"))
  ;[0.05098 0.05098 0.05098] Normalizes an input angle into a valid range of 0 to 360 degrees
  (return (`KismetMathLibrary.SelectFloat` (mod (+ (`local.In`) 360.0) 360.0) (`local.In`) (< (`local.In`) 0.0))))

(fn `ConvertToTranslation`
  (params (A :type "Rotator Structure") (B :type "Rotator Structure"))
  (returns (Translation :type "Vector2D Structure") (`IsClockwise?` :type Boolean) (`IsInRadarLength?` :type Boolean))
  (bind _returnvalue (`self.ConvertToCircleDegrees` (.yaw (`local.B`))))
  (bind _returnvalue_2 (`self.ConvertToCircleDegrees` (.yaw (`local.A`))))
  (bind _returnvalue_3 (`self.GetDelta` _returnvalue_2 _returnvalue))
  (bind _returnvalue_4 (`self.GetDelta` _returnvalue_2 _returnvalue true))
  (bind _returnvalue_5 (/ _returnvalue_3 (`CameraComponent.FieldOfView` (`self.PlayerCamera`))))
  (bind _returnvalue_6 (/ _returnvalue_4 (`CameraComponent.FieldOfView` (`self.PlayerCamera`))))
  (bind _returnvalue_7 (<= _returnvalue_6 1.0))
  (bind _returnvalue_8 (<= _returnvalue_5 1.0))
  ;[0.05098 0.05098 0.05098] Computes the translation of two input rotations into a spatial representation - accounts for angular deltas, field of view constraints, and radar length clamping to calculate the values
  (`/Engine/EditorBlueprintResources/StandardMacros.CompareFloat` _returnvalue_4 _returnvalue_3
    (:`>`
      (return (`KismetMathLibrary.MakeVector2D` (`KismetMathLibrary.SelectFloat` (* (`KismetMathLibrary.Lerp` 0.0 (`self.RadarClampLength`) _returnvalue_5) -1.0) 0.0 _returnvalue_8)) false (select `bool` _returnvalue_8 :`true` true)))
    (:`==`
      _)
    (:`<`
      _))
  (return (`KismetMathLibrary.MakeVector2D` (`KismetMathLibrary.SelectFloat` (`KismetMathLibrary.Lerp` 0.0 (`self.RadarClampLength`) _returnvalue_6) 0.0 _returnvalue_7)) true (select `bool` _returnvalue_7 :`true` true)))

(fn `GetDelta`
  (params (A :type "Float (double-precision)") (B :type "Float (double-precision)") (`IsClockwise?` :type Boolean))
  (returns (ReturnValue :type "Float (double-precision)"))
  (locals (LOCAL_A :type "Float (double-precision)" :default 0.0) (LOCAL_B :type "Float (double-precision)" :default 0.0))
  ;[0.05098 0.05098 0.05098] Calculates the delta between two angular. Also determines the appropriate output based on whether the difference should be interpreted as clockwise or counterclockwise
  (set `local.LOCAL_A` (mod A 360.0))
  (set `local.LOCAL_B` (mod B 360.0))
  (`/Engine/EditorBlueprintResources/StandardMacros.CompareFloat` (`local.LOCAL_A`) (`local.LOCAL_B`)
    (:`>`
      (return (`KismetMathLibrary.SelectFloat` (- 360.0 (- (`local.LOCAL_A`) (`local.LOCAL_B`))) (- (`local.LOCAL_A`) (`local.LOCAL_B`)) (`local.IsClockwise?`))))
    (:`==`
      (return 0.0))
    (:`<`
      (return (`KismetMathLibrary.SelectFloat` (- (`local.LOCAL_B`) (`local.LOCAL_A`)) (- 360.0 (- (`local.LOCAL_B`) (`local.LOCAL_A`))) (`local.IsClockwise?`))))))

(fn `RefreshCardinals`
  (locals (LOCAL_CardinalData :type "Array of /Game/SoulslikeFramework/Structures/Compass/FCardinalData Structure") (LOCAL_CardinalEntry :type "/Game/SoulslikeFramework/Widgets/Radar/W_Radar_Cardinal Object Reference"))
  ;[0.05098 0.05098 0.05098] Foreach cardinal entry
  (bind _values (`BlueprintMapLibrary.Map_Values` (`self.CardinalData`)))
  (set `local.LOCAL_CardinalData` _values)
  (bind _radarwidget (`self.RadarWidget`)
    (:`then`
      (for (_array_element _array_index) (`/Game/SoulslikeFramework/Widgets/Radar/W_Radar.Cardinals` _radarwidget)
        ;[0.05098 0.05098 0.05098] Convert from world to 2d translation and update render translation of the entry.
        (set `local.LOCAL_CardinalEntry` _array_element)
        (bind (_translation _isclockwise_ _isinradarlength_) (`self.ConvertToTranslation` (`SceneComponent.K2_GetComponentRotation` (`self.PlayerCamera`)) (`KismetMathLibrary.MakeRotator` 0.0 0.0 (`.Value_6_63F84C6F4A9F0ABD65FD7AA9514E1721` (break `/Game/SoulslikeFramework/Structures/Compass/FCardinalData` (`|GetArrayItem` (`local.LOCAL_CardinalData`) _array_index))))))
        (if _isinradarlength_
          (`Widget.SetRenderTranslation` (`local.LOCAL_CardinalEntry`) _translation)
          ;[0.05098 0.05098 0.05098] Adjust visibility
          (`Widget.SetVisibility` (`local.LOCAL_CardinalEntry`) (select `bool` (`Widget.IsVisible` (`local.LOCAL_CardinalEntry`)) :`false` "Visible" :`true` "Visible" :!type "ESlateVisibility Enum"))
          (else
            (`Widget.SetVisibility` (`local.LOCAL_CardinalEntry`) (select `bool` (`Widget.IsVisible` (`local.LOCAL_CardinalEntry`)) :`false` "Collapsed" :`true` "Collapsed" :!type "ESlateVisibility Enum"))))))
    (:`else`)))

(fn `RefreshTrackedElements`
  (locals (LOCAL_MarkerWidget :type "/Game/SoulslikeFramework/Widgets/Radar/W_Radar_TrackedElement Object Reference"))
  (`self.RadarWidget`
    (:`then`
      (for _array_element (`self.TrackedComponents`)
        (`/Engine/EditorBlueprintResources/StandardMacros.IsValid` _array_element
          (:`Is Valid`
            (bind _markerwidget (`/Game/SoulslikeFramework/Blueprints/Components/AC_RadarElement.MarkerWidget` _array_element)
              (:`then`
                (set `local.LOCAL_MarkerWidget` _markerwidget)
                (bind (_translation _isclockwise_ _isinradarlength_) (`self.ConvertToTranslation` (`SceneComponent.K2_GetComponentRotation` (`self.PlayerCamera`)) (`KismetMathLibrary.FindLookAtRotation` (`Actor.K2_GetActorLocation` (`self.Pawn`)) (`Actor.K2_GetActorLocation` (`self.GetOwner` _array_element)))))
                (if _isinradarlength_
                  (`Widget.SetRenderTranslation` (`local.LOCAL_MarkerWidget`) _translation)
                  ;[0.05098 0.05098 0.05098] Adjust visibility
                  (`Widget.SetVisibility` (`local.LOCAL_MarkerWidget`) (select `bool` (`Widget.IsVisible` (`local.LOCAL_MarkerWidget`)) :`false` "Visible" :`true` "Visible" :!type "ESlateVisibility Enum"))
                  (else
                    (`Widget.SetVisibility` (`local.LOCAL_MarkerWidget`) (select `bool` (`Widget.IsVisible` (`local.LOCAL_MarkerWidget`)) :`false` "Collapsed" :`true` "Collapsed" :!type "ESlateVisibility Enum")))))
              (:`else`))))))
    (:`else`)))

(fn `SetupCardinals`
  ;[0.05098 0.05098 0.05098] Foreach cardinal entry, add a cardinal widget
  (`self.RadarWidget`
    (:`then`
      (bind _values (`BlueprintMapLibrary.Map_Values` (`self.CardinalData`)))
      (for _array_element _values
        (`/Game/SoulslikeFramework/Widgets/Radar/W_Radar.AddCardinal` (`self.RadarWidget`) _array_element 2))
      (`self.RefreshCardinals`))
    (:`else`)))

(fn `SetupPlayerIcon`
  ;[0.05098 0.05098 0.05098] Sets player icon and its scale/tint
  (bind _radarwidget (`self.RadarWidget`)
    (:`then`
      (`/Game/SoulslikeFramework/Widgets/Radar/W_Radar.SetPlayerIcon` _radarwidget (`self.PlayerIcon`) (`self.IconTint`) (`self.IconSize`)))
    (:`else`)))

(fn `StartTrackElement`
  (params (TrackedElement :type "/Game/SoulslikeFramework/Blueprints/Components/AC_RadarElement Object Reference"))
  (returns (TrackedElementWidget :type "/Game/SoulslikeFramework/Widgets/Radar/W_Radar_TrackedElement Object Reference"))
  (bind _trackedelement (`local.TrackedElement`))
  ;[0.05098 0.05098 0.05098] Starts tracking element. Target actor must have an AC_RadarElement component.
  (if (not (`KismetArrayLibrary.Array_Contains` (`self.TrackedComponents`) TrackedElement))
    (`KismetArrayLibrary.Array_Add` (`self.TrackedComponents`) (`local.TrackedElement`))
    (bind _radarwidget (`self.RadarWidget`)
      (:`then`
        (bind _trackedelementwidget (`/Game/SoulslikeFramework/Widgets/Radar/W_Radar.AddTrackedElement` _radarwidget (`/Game/SoulslikeFramework/Blueprints/Components/AC_RadarElement.Icon` _trackedelement) (`/Game/SoulslikeFramework/Blueprints/Components/AC_RadarElement.IconTint` _trackedelement) (`/Game/SoulslikeFramework/Blueprints/Components/AC_RadarElement.IconSize` _trackedelement)))
        (return _trackedelementwidget))
      (:`else`))
    (else
      (return null))))

(fn `StopTrackElement`
  (params (Element :type "/Game/SoulslikeFramework/Blueprints/Components/AC_RadarElement Object Reference"))
  ;[0.05098 0.05098 0.05098] Stops tracking element. Target actor must have an AC_RadarElement component.
  (if (`KismetArrayLibrary.Array_Contains` (`self.TrackedComponents`) Element)
    (`KismetArrayLibrary.Array_RemoveItem` (`self.TrackedComponents`) (`local.Element`))
    (bind _markerwidget (`/Game/SoulslikeFramework/Blueprints/Components/AC_RadarElement.MarkerWidget` (`local.Element`))
      (:`then`
        (bind _radarwidget (`self.RadarWidget`)
          (:`then`
            (`/Game/SoulslikeFramework/Widgets/Radar/W_Radar.RemoveTrackedElement` _radarwidget _markerwidget))
          (:`else`)))
      (:`else`))))

(fn `ToggleUpdateState`
  (params (`ShouldUpdate?` :type Boolean))
  (bind _timer (`self.Timer`))
  ;[0.05098 0.05098 0.05098] Enable/disable radar's update functionality. Will basically pause the radar.
  (bind _output_get (set `self.ShouldUpdate?` `ShouldUpdate?`))
  (if _output_get
    (if (`self.Visible?`)
      (`KismetSystemLibrary.K2_UnPauseTimerHandle` _timer)
      (else
        (`KismetSystemLibrary.K2_PauseTimerHandle` _timer)))))