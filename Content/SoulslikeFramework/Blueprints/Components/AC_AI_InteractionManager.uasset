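; AI interaction component for the Soulslike Framework that runs NPC dialog and hands off to vendor windows.
; Each BeginDialog call async-loads the DialogAsset table matching player progress, resetting the index when the table changes.
; It fires the entry's gameplay events through the progress manager and sends text to the HUD, ending in vendor setup or dialog finish.
; Separate events correct the index on exit or reset it.
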(event `Event BeginDialog`
  (params (ProgressManager :type "/Game/SoulslikeFramework/Blueprints/Components/AC_ProgressManager Object Reference") (HUD :type "/Game/SoulslikeFramework/Widgets/HUD/W_HUD Object Reference"))
  ;[0.05098 0.05098 0.05098] Ensure that we have a valid reference to player's progress manager & the NPC's dialog asset.
  (`/Engine/EditorBlueprintResources/StandardMacros.IsValid` ProgressManager
    (:`Is Valid`
      (set `self.ProgressManager` ProgressManager)
      (`self.DialogAsset`
        (:`then`
          ;[0.05098 0.05098 0.05098] Get appropriate Dialog Table based on players progress and reset talk index to 0.
          (bind _table (`/Game/SoulslikeFramework/Data/Dialog/PDA_Dialog.GetDialogTableBasedOnProgress` (`self.DialogAsset`) (`self.ProgressManager`)))
          (if (!= (`self.ActiveTable`) _table)
            (set `self.CurrentIndex` 0))
          (bind _output_get (set `self.ActiveTable` _table))
          ;[0.05098 0.05098 0.05098] Execute dialog logic. If current dialog entry has an event, execute the gameplay event (see more inside AC_ProgressManager -> ExecuteGameplayEvent()). Adjust index accordingly and set text or exit dialog.
          (bind _object (`|LoadAsset` _output_get)
            (:`Completed`
              (bind _asdata_table (cast `DataTable` _object))
              (bind _outrownames (`DataTableFunctionLibrary.GetDataTableRowNames` _asdata_table))
              (bind _out_row (`self.GetCurrentDialogEntry` _asdata_table _outrownames))
              (bind _returnvalue (`KismetArrayLibrary.Array_Length` _outrownames))
              (set `self.MaxIndex` (- _returnvalue 1))
              (bind (_entry _gameplayevents) (break `/Game/SoulslikeFramework/Structures/Dialog/FDialogEntry` _out_row))
              (`/Game/SoulslikeFramework/Blueprints/Components/AC_ProgressManager.ExecuteGameplayEvents` (`self.ProgressManager`) _gameplayevents)
              (bind _returnvalue_2 (+ _returnvalue 1))
              (bind _output_get_2 (set `self.CurrentIndex` (`KismetMathLibrary.Clamp` (+ (`self.CurrentIndex`) 1) 0 _returnvalue_2)))
              (if (== _output_get_2 _returnvalue_2)
                (set `self.CurrentIndex` (- _output_get_2 2))
                ;[0.05098 0.05098 0.05098] After last dialog index, if vendor asset is valid, setup NPC window
                (bind _vendorasset (`self.VendorAsset`)
                  (:`then`
                    (`/Game/SoulslikeFramework/Widgets/HUD/W_HUD.Event SetupNpcWindow` HUD (`self.Name`) _vendorasset self))
                  (:`else`
                    (`/Game/SoulslikeFramework/Widgets/HUD/W_HUD.Event FinishDialog` HUD)
                    (`self.OnDialogFinished`)))
                (else
                  (`/Game/SoulslikeFramework/Widgets/HUD/W_HUD.Event SetupDialog` HUD _entry))))))
        (:`else`)))))

(event `Event AdjustIndexForExit`
  (bind _currentindex (`self.CurrentIndex`))
  ;[0.05098 0.05098 0.05098] Adjust index if player exits dialog mid-way
  (bind _activetable (`self.ActiveTable`)
    (:`then`
      (bind _object (`|LoadAsset` _activetable)
        (:`Completed`
          (bind _asdata_table (cast `DataTable` _object))
          (bind _outrownames (`DataTableFunctionLibrary.GetDataTableRowNames` _asdata_table))
          (if (== (`KismetArrayLibrary.Array_Length` _outrownames) _currentindex)
            (set `self.CurrentIndex` (- _currentindex 1))))))
    (:`else`)))

(event `Event ResetDialogIndex`
  ;[0.05098 0.05098 0.05098] Method to reset dialog index to 0.
  (`self.DialogAsset`
    (:`then`
      (set `self.CurrentIndex` 0))
    (:`else`)))

(fn `GetCurrentDialogEntry`
  (params (DataTable :type "DataTable Object Reference") (Rows :type "Array of Name"))
  (returns (`Out Row` :type "/Game/SoulslikeFramework/Structures/Dialog/FDialogEntry Structure"))
  ;[0.05098 0.05098 0.05098] Returns current dialog entry
  (bind _returnvalue (`|GetDataTableRow` DataTable (`|GetArrayItem` Rows (`self.CurrentIndex`)))
    (:`then`
      (return _returnvalue))))