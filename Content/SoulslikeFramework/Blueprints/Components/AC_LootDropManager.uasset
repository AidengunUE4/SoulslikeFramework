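; Loot drop component that chooses an item to drop and announces it through OnItemReadyForSpawn, leaving the spawning to other code.
; PickItem async-loads the LootTable DataTable and makes a weighted random pick by summing row weights and subtracting through the entries.
; A valid OverrideItem replaces the rolled result, and OverrideItem is also sent directly when no loot table is set.
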(event `Event PickItem`
  ;[0.05098 0.05098 0.05098] Picks a random item from the provided table.
  (bind _loot_table (`self.Loot Table`)
    (:`then`
      (bind _object (`|LoadAsset` _loot_table)
        (:`Completed`
          (bind _asdata_table (cast `DataTable` _object))
          (bind _selecteditem (`self.GetRandomItemFromTable` _asdata_table))
          (`self.OnItemReadyForSpawn` (select `bool` (`self.IsOverrideItemValid?`) :`false` _selecteditem :`true` (`self.Override Item`))))))
    (:`else`
      (`self.OnItemReadyForSpawn` (`self.Override Item`)))))

(fn `GetRandomItemFromTable`
  (params (LootTable :type "DataTable Object Reference"))
  (returns (SelectedItem :type "/Game/SoulslikeFramework/Structures/_Misc/FLootItem Structure"))
  (locals (LOCAL_Items :type "Map of /Game/SoulslikeFramework/Structures/_Misc/FLootItem Structure to Float (double-precision)") (LOCAL_Value :type "Float (double-precision)") (LOCAL_Score :type "Float (double-precision)"))
  ;[0.05098 0.05098 0.05098] Selects item from the table based on its weight.
  (`/Engine/EditorBlueprintResources/StandardMacros.IsValid` LootTable
    (:`Is Valid`
      (bind _outrownames (`DataTableFunctionLibrary.GetDataTableRowNames` LootTable))
      (for _array_element _outrownames
        (bind _returnvalue (`|GetDataTableRow` (`local.LootTable`) _array_element)
          (:`then`
            (bind (_item _weight) (break `/Game/SoulslikeFramework/Structures/_Misc/FWeightedLoot` _returnvalue))
            (`BlueprintMapLibrary.Map_Add` (`local.LOCAL_Items`) _item _weight)
            (set `local.LOCAL_Score` (+ (`local.LOCAL_Score`) _weight)))))
      (set `local.LOCAL_Value` (`KismetMathLibrary.RandomFloatInRange` 0.0 (`local.LOCAL_Score`)))
      (bind _keys (`BlueprintMapLibrary.Map_Keys` (`local.LOCAL_Items`)))
      (for _array_element_2 _keys
        (bind _value (`BlueprintMapLibrary.Map_Find` (`local.LOCAL_Items`) _array_element_2))
        (if (< (`local.LOCAL_Value`) _value)
          (return _array_element_2)
          (else
            (set `local.LOCAL_Value` (- (`local.LOCAL_Value`) _value))))))))

(fn `IsOverrideItemValid?`
  (returns (ReturnValue :type Boolean))
  ;[0.05098 0.05098 0.05098] Checks if there's an override item
  (return (`KismetSystemLibrary.IsValid` (`.Item_2_0AA5E0034E8F2A92CFB8589C26666176` (break `/Game/SoulslikeFramework/Structures/_Misc/FLootItem` (`self.Override Item`))))))