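; Player controller for the Soulslike Framework that owns the HUD and fronts radar, inventory, progress and save/load components.
; Menu input actions route to the HUD widget matching the active gameplay tag, and input mapping contexts swap per game state.
; Death fades to a loading screen, moves the pawn to the last resting point (fallbacks: nearest activated, PlayerStart), resets stats and saves.
; Save completion reloads the saved level if that loading screen exists.
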(fn `GetCurrency`
  (returns (Currency :type Integer))
  (return (`/Game/SoulslikeFramework/Blueprints/Components/AC_InventoryManager.GetCurrentCurency` (`self.AC_InventoryManager`))))

(fn `GetInventoryComponent`
  (returns (Inventory :type "/Game/SoulslikeFramework/Blueprints/Components/AC_InventoryManager Object Reference"))
  (bind _ac_inventorymanager (`self.AC_InventoryManager`)
    (:`then`
      (return _ac_inventorymanager))
    (:`else`)))

(fn `GetNearestRestingPoint`
  (returns (Success :type Boolean) (Point :type "Actor Object Reference"))
  (locals (LOCAL_Distance :type Boolean))
  ;[0.05098 0.05098 0.05098] Returns nearest resting point actor of class B_RestingPoint.
  (bind _outactors (`GameplayStatics.GetAllActorsOfClass` "/Game/SoulslikeFramework/Blueprints/_WorldActors/Interactables/B_RestingPoint.B_RestingPoint_C"))
  (bind (_distance _returnvalue) (`GameplayStatics.FindNearestActor` (`self.K2_GetActorLocation` (`self.K2_GetPawn`)) _outactors))
  (`/Engine/EditorBlueprintResources/StandardMacros.IsValid` _returnvalue
    (:`Is Valid`
      (return true _returnvalue))
    (:`Is Not Valid`
      (return false null))))

(fn `GetPawnFromController`
  (returns (Pawn :type "Pawn Object Reference"))
  (return (`self.K2_GetPawn`)))

(fn `GetPlayerHUD`
  (returns (W_HUD :type "/Game/SoulslikeFramework/Widgets/HUD/W_HUD Object Reference"))
  (return (`self.W_HUD`)))

(fn `GetProgressManager`
  (returns (ProgressManager :type "/Game/SoulslikeFramework/Blueprints/Components/AC_ProgressManager Object Reference"))
  (return (`self.AC_ProgressManager`)))

(fn `GetSoulslikeController`
  (returns (PC_SoulslikeFramework :type "/Game/SoulslikeFramework/Blueprints/Global/PC_SoulslikeFramework Object Reference"))
  (return self))

(fn `Handle Main Menu Request`
  ;[0.05098 0.05098 0.05098] If Dialog Window is active, first finish dialog. Then on the second press, show game menu.
  (`self.W_HUD`
    (:`then`
      (`|ExecutionSequence`
        (:`then_0`
          (if (`/Game/SoulslikeFramework/Widgets/HUD/W_HUD.GetDialogWindowVisibility` (`self.W_HUD`))
            (`/Game/SoulslikeFramework/Widgets/HUD/W_HUD.Event FinishDialog` (`self.W_HUD`))
            (return)))
        (:`then_1`
          (if (not (`/Game/SoulslikeFramework/Widgets/HUD/W_HUD.GetGameMenuVisibility` (`self.W_HUD`)))
            (`/Game/SoulslikeFramework/Widgets/HUD/W_HUD.Event ShowGameMenu` (`self.W_HUD`))
            (return)))))
    (:`else`)))

(fn `UserConstructionScript`)