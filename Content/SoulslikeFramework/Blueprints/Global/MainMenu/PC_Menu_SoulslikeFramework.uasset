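; Player controller for the Soulslike Framework main menu, creating the menu widget and routing navigation input to it.
; BeginPlay adds the menu input mapping, asks the game instance whether any save exists, then creates W_MainMenu with that as CanContinueGame.
; Enhanced Input actions switch on an active-widget gameplay tag to forward navigation to main menu, credits, settings, character select or load slots.
; Controller getter functions are empty stubs.
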(fn `GetCurrency`
  (returns (Currency :type Integer))
  (return 0))

(fn `GetInventoryComponent`
  (returns (Inventory :type "/Game/SoulslikeFramework/Blueprints/Components/AC_InventoryManager Object Reference"))
  (return null))

(fn `GetPawnFromController`
  (returns (Pawn :type "Pawn Object Reference"))
  (return null))

(fn `GetPlayerHUD`
  (returns (W_HUD :type "/Game/SoulslikeFramework/Widgets/HUD/W_HUD Object Reference"))
  (return null))

(fn `GetProgressManager`
  (returns (ProgressManager :type "/Game/SoulslikeFramework/Blueprints/Components/AC_ProgressManager Object Reference"))
  (return null))

(fn `GetSoulslikeController`
  (returns (PC_SoulslikeFramework :type "/Game/SoulslikeFramework/Blueprints/Global/PC_SoulslikeFramework Object Reference"))
  (return null))

(fn `UserConstructionScript`)