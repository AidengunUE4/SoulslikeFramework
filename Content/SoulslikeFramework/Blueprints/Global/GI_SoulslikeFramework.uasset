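; Game instance for the Soulslike Framework that tracks save slots, the active slot and the selected character class across the game.
; On Init it loads the slot-tracker save object, or creates one if none exists.
; New slots are added to that object and saved asynchronously, and the active slot can be set directly or to the last saved one.
; Class changes notify listeners, and getters expose slots, class and custom game settings.
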(event `self.ReceiveInit`
  ;[0.05098 0.05098 0.05098] Create and maintain Slot tracker save game object.
  (bind _returnvalue (`GameplayStatics.DoesSaveGameExist` (`self.SlotsSaveName`)))
  (if _returnvalue
    (bind _returnvalue_2 (`GameplayStatics.LoadGameFromSlot` (`self.SlotsSaveName`)))
    (bind _assg_save_slots (cast `/Game/SoulslikeFramework/Blueprints/Saving/SG_SaveSlots` _returnvalue_2))
    (set `self.SGO_Slots` _assg_save_slots)
    (else
      (`self.SGO_Slots`
        (:`then`)
        (:`else`
          (bind _returnvalue_3 (`GameplayStatics.CreateSaveGameObject` "/Game/SoulslikeFramework/Blueprints/Saving/SG_SaveSlots.SG_SaveSlots_C"))
          (set `self.SGO_Slots` _returnvalue_3))))))

(event `/Game/SoulslikeFramework/Blueprints/Interfaces/BPI_GameInstance.SetSelectedClass`
  (params (BaseCharacterClass :type "/Game/SoulslikeFramework/Data/PDA_BaseCharacterInfo Object Reference"))
  ;[0.05098 0.05098 0.05098] Change class and notify listeners
  (set `self.SelectedBaseClass` BaseCharacterClass)
  (`self.OnSelectedClassChanged`))

(event `/Game/SoulslikeFramework/Blueprints/Interfaces/BPI_GameInstance.SetActiveSlot`
  (params (ActiveSlotName :type String))
  ;[0.05098 0.05098 0.05098] Set active Save Slot name
  (set `self.ActiveSlot` ActiveSlotName))

(event `/Game/SoulslikeFramework/Blueprints/Interfaces/BPI_GameInstance.AddAndSaveSlots`
  (params (NewSlotName :type String))
  ;[0.05098 0.05098 0.05098] Add new save slot and save
  (`/Game/SoulslikeFramework/Blueprints/Saving/SG_SaveSlots.AddSlot` (`self.SGO_Slots`) NewSlotName)
  (`AsyncActionHandleSaveGame.AsyncSaveGameToSlot` (`self.SGO_Slots`) (`self.SlotsSaveName`)
    (:`Completed`
      (`KismetSystemLibrary.PrintText` (`|FormatText` "\"{slot}\" has been added to slots list." NewSlotName)))))

(event `/Game/SoulslikeFramework/Blueprints/Interfaces/BPI_GameInstance.SetLastSlotNameToActive`
  ;[0.05098 0.05098 0.05098] Set Active Slot to be last saved slot
  (bind _sgo_slots (`self.SGO_Slots`)
    (:`then`
      (set `self.ActiveSlot` (`/Game/SoulslikeFramework/Blueprints/Saving/SG_SaveSlots.GetLastSaveSlot` _sgo_slots)))
    (:`else`)))

(fn `DoesAnySaveExist?`
  (returns (ReturnValue :type Boolean))
  (bind _returnvalue (`GameplayStatics.DoesSaveGameExist` (`self.SlotsSaveName`)))
  (return _returnvalue))

(fn `GetActiveSlotName`
  (returns (ActiveSlotName :type String))
  (return (`self.ActiveSlot`)))

(fn `GetAllSaveSlots`
  (returns (SaveSlots :type "Array of String"))
  (bind _sgo_slots (`self.SGO_Slots`)
    (:`then`
      (bind _slots (`/Game/SoulslikeFramework/Blueprints/Saving/SG_SaveSlots.GetAllSlots` _sgo_slots))
      (return _slots))
    (:`else`)))

(fn `GetCustomGameSettings`
  (returns (CustomSettingsAsset :type "/Game/SoulslikeFramework/Data/PDA_CustomSettings Object Reference"))
  (return (`self.CustomGameSettings`)))

(fn `GetSelectedClass`
  (returns (SelectedBaseCharacterClass :type "/Game/SoulslikeFramework/Data/PDA_BaseCharacterInfo Object Reference"))
  (return (`self.SelectedBaseClass`)))

(fn `GetSoulslikeGameInstance`
  (returns (ReturnValue :type "/Game/SoulslikeFramework/Blueprints/Global/GI_SoulslikeFramework Object Reference"))
  (return self))