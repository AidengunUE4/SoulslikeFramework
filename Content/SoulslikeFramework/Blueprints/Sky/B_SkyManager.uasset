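; Sky manager actor that runs a day/night cycle for the Soulslike framework.
; Tick advances a 24-hour clock scaled by TimeDilation, rotating opposed sun and moon lights and setting height fog density from a curve.
; A one-second timer refreshes the current time entry from a data asset.
; Interior/exterior lighting modes animate fog start distance to stop fog leaking through walls, and the Construction Script previews the sky in editor.
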(event `self.ReceiveBeginPlay`
  ;[0.05098 0.05098 0.05098] On BeginPlay, start a time-check method on a 1 sec interval and switch lightning mode to desired lightning mode.
  (`KismetSystemLibrary.K2_SetTimerDelegate` (`|CreateDelegate` :!event `Event CheckTimeInfo`) 1.0 true)
  (`self.Event SwitchLightningMode` (`self.CurrentLightningMode`)))

(event `self.ReceiveTick`
  (params (DeltaSeconds :type "Float (single-precision)"))
  (bind _returnvalue (* (/ (`self.Time`) 24.0) 360.0))
  ;[0.05098 0.05098 0.05098] Simple Day/Night cycle. Rotate Sun & Moon directional lights. Adjust exponential height fog density using the float curve track.
  (bind _output_get (set `self.Time` (+ (/ DeltaSeconds (`self.TimeDilation`)) (`self.Time`))))
  (if (>= _output_get 24.0)
    (set `self.Time` 0.0)
    (else
      (`SceneComponent.K2_SetRelativeRotation` (`self.DirectionalLight_Sun`) (`KismetMathLibrary.MakeRotator` 0.0 _returnvalue) false false)
      (`SceneComponent.K2_SetRelativeRotation` (`self.DirectionalLight_Moon`) (`KismetMathLibrary.MakeRotator` 0.0 (+ _returnvalue 180.0)) false false)
      (`ExponentialHeightFogComponent.SetFogDensity` (`self.ExponentialHeightFog`) (`CurveFloat.GetFloatValue` (`self.FogDensityTrack`) (`self.Time`))))))

(event `Event CheckTimeInfo`
  ;[0.05098 0.05098 0.05098] Set time entry info - this is run on a 1 sec interval.
  (bind _timeentry (`/Game/SoulslikeFramework/Data/PDA_DayNight.GetEntryForTime` (`self.TimeInfoAsset`) (`self.Time`)))
  (set `self.TimeEntryInfo` _timeentry))

(event `Event AdjustTime`
  (params (TargetTime :type "Float (double-precision)"))
  ;[0.05098 0.05098 0.05098] Simple method to adjust current time.
  (set `self.Time` TargetTime))

(event `Event SwitchLightningMode`
  (params (NewLightningMode :type "/Game/SoulslikeFramework/Enums/E_LightningMode Enum" :default "NewEnumerator0"))
  ;[0.05098 0.05098 0.05098] Simple method to switch lightning mode. Support interior/exterior lightning which adjusts the exponential height fog's start distance to combat fog leaking through walls.
  (bind _output_get (set `self.CurrentLightningMode` NewLightningMode))
  (switch `/Game/SoulslikeFramework/Enums/E_LightningMode` _output_get
    (:`NewEnumerator0`
      (bind (_direction _alpha) (`Timeline|FogExterior` :!via `PlayFromStart` :!label _label)
        (:`Update`
          (`ExponentialHeightFogComponent.SetStartDistance` (`self.ExponentialHeightFog`) (`KismetMathLibrary.Lerp` 10000.0 0.0 _alpha)))))
    (:`NewEnumerator1`
      (goto _label :!via `ReverseFromEnd`))))

(fn `UserConstructionScript`
  (bind _returnvalue (* (/ (`self.Time`) 24.0) 360.0))
  ;[0.05098 0.05098 0.05098] Switch Lightning Mode, set relative rotation of Sun/Moon, and set Fog Density on construction for viewing purposes.
  (`self.Event SwitchLightningMode` (`self.CurrentLightningMode`))
  (`SceneComponent.K2_SetRelativeRotation` (`self.DirectionalLight_Sun`) (`KismetMathLibrary.MakeRotator` 0.0 _returnvalue) false false)
  (`SceneComponent.K2_SetRelativeRotation` (`self.DirectionalLight_Moon`) (`KismetMathLibrary.MakeRotator` 0.0 (+ _returnvalue 180.0)) false false)
  (`ExponentialHeightFogComponent.SetFogDensity` (`self.ExponentialHeightFog`) (`CurveFloat.GetFloatValue` (`self.FogDensityTrack`) (`self.Time`))))